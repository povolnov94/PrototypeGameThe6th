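; BP_DmgAmount is a floating damage number actor that shows a hit amount in the world.
; On BeginPlay it passes its DmgAmount to the WBP_DamageValue widget in its widget component.
; A timeline then lerps the actor from its start location to a fixed raised, slightly sideways world offset, and destroys it when finished.
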(event EventBeginPlay
  (bind _aswbp_damage_value (Utilities|Casting|CastToWBP_DamageValue (UserInterface|GetWidget (Variables|Default|GetWidget))))
  (Variables|/Game/HUD/WBP_DamageValue.WBP_DamageValue_C|SetDmgAmount _aswbp_damage_value (Variables|Default|GetDmg%20Amount))
  (bind _output_get (Variables|Default|SetStartLocation (Transformation|GetActorLocation)))
  (Variables|Default|SetEndLocation (+ _output_get "-25.000000,-25.000000,50.000000"))
  (bind _movetrack (Timeline|MoveT Play)
    (:Update
      (Transformation|SetActorLocation (Math|Vector|Lerp(Vector) (Variables|Default|GetStartLocation) (Variables|Default|GetEndLocation) _movetrack) false false))
    (:Finished
      (Actor|DestroyActor))))

(fn ConstructionScript)