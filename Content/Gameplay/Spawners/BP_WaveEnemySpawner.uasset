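; Wave enemy spawner that queues enemy classes and spawns them at its own transform.
; Once activated, it retries every few seconds, while newly queued enemies also trigger an immediate spawn if its sphere has no overlapping enemies.
; It binds to each spawn's killed event and has a handler relaying kills to the game mode.
; At wave end, it sets its on flag by comparing the next wave number to its activation round.
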(event Custom|OnEnemyKilled
  (bind _asbp_third_person_game_mode (Utilities|Casting|CastToBP_ThirdPersonGameMode (Game|GetGameMode)))
  (Default|OnEnemyKilled _asbp_third_person_game_mode))

(event Custom|TryToSpawn
  (CallFunction|SpawnEnemy))

(event Custom|OnEndWave
  (Variables|Default|SetIsSpawnerOn (>= (+ (Variables|/Game/ThirdPerson/Blueprints/BP_ThirdPersonGameMode.BP_ThirdPersonGameMode_C|GetWaveNumber (Variables|Default|GetThirdPersonGameMode)) 1) (Variables|Default|GetRoundActivated))))

(event Custom|Activate
  (Utilities|Time|SetTimerbyEvent (delegate Custom|TryToSpawn) 3.0 true)
  (bind _asbp_third_person_game_mode (Utilities|Casting|CastToBP_ThirdPersonGameMode (Game|GetGameMode)))
  (bind _output_get (Variables|Default|SetThirdPersonGameMode _asbp_third_person_game_mode))
  (EventDispatchers|BindEventtoOnEndWave _output_get (delegate Custom|OnEndWave)))

(event EventBeginPlay)

(fn ConstructionScript)

(fn SpawnEnemy
  (if (Utilities|Array|IsValidIndex (Variables|Default|GetEnemyQueue))
    (bind _returnvalue (Game|SpawnActorfromClass (Utilities|Array|Get(acopy) (Variables|Default|GetEnemyQueue)) (Transformation|GetActorTransform) "AdjustIfPossibleButAlwaysSpawn" "MultiplyWithRoot" 0 0))
    (if (Utilities|IsValid _returnvalue)
      (EventDispatchers|BindEventtoOnKilled _returnvalue (EventDispatchers|CreateEvent :!event Custom|OnEnemyKilled))
      (Utilities|Array|RemoveIndex (Variables|Default|GetEnemyQueue))
      (return true))
    (else
      (return false))))

(fn AddEnemytoQueue
  (params (EnemyClass :type BP%20Enemy%20Base%20Class%20Reference%20%28by%20ref%29))
  (Utilities|Array|Add (Variables|Default|GetEnemyQueue) EnemyClass)
  (if (not (Utilities|Array|IsValidIndex (Collision|GetOverlappingActors (Variables|Default|GetSphere) "/Game/Enemy/BP_EnemyBase.BP_EnemyBase_C" :!class /Script/Engine.PrimitiveComponent)))
    (CallFunction|SpawnEnemy)))