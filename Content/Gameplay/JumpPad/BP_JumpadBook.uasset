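; Jump pad actor that launches player 0 when its Box is overlapped, unless hidden.
; Launch velocity comes from a suggested projectile arc toward ForceVector rotated by actor rotation, applied as a velocity-change impulse.
; Options zero the player's velocity before launch or move them above the pad afterwards.
; With DrawEditorLines, the construction script predicts the projectile path and spawns arrow components along it as a preview.
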(event OnComponentBeginOverlap(Box)
  (params (OverlappedComponent :type Primitive%20Component%20Object%20Reference) (OtherActor :type Actor%20Object%20Reference) (OtherComp :type Primitive%20Component%20Object%20Reference) (OtherBodyIndex :type Integer) (bFromSweep :type Boolean) (SweepResult :type Hit%20Result%20Structure%20%28by%20ref%29))
  (if (not (Variables|Rendering|GetbHidden))
    (if (Variables|Default|GetIsPlayerVelocityIgnored)
      (Variables|/Script/Engine.MovementComponent|SetVelocity (Variables|/Script/Engine.Character|GetCharacterMovement (Game|GetPlayerCharacter 0)) "0, 0, 0"))
    (bind _launchvelocity (CallFunction|CalcLaunchVelocity))
    (Physics|AddImpulse (Variables|/Script/Engine.Character|GetCharacterMovement (Game|GetPlayerCharacter 0)) _launchvelocity true)
    (if (Variables|Default|GetAdjustPlayerPosition)
      (Transformation|SetActorLocation (Game|GetPlayerCharacter 0) (+ (Transformation|GetActorLocation) "0.000000,0.000000,200.000000") false false))))

(event EventBeginPlay)

(event Collision|EventActorBeginOverlap
  (params (OtherActor :type Actor%20Object%20Reference)))

(event EventTick
  (params (DeltaSeconds :type Float%20%28single-precision%29)))

(fn ConstructionScript
  (if (Variables|Default|GetDrawEditorLines)
    (bind _launchvelocity (CallFunction|CalcLaunchVelocity))
    (CallFunction|CreateLaunchArk _launchvelocity)))

(fn CalcLaunchVelocity
  (bind _outlaunchvelocity (Game|SuggestProjectileVelocityCustomArc "0, 0, 0" (Math|Vector|RotateVector (Variables|Default|GetForceVector) (Transformation|GetActorRotation)) 0.0 0.5))
  (return true _outlaunchvelocity))

(fn CreateLaunchArk
  (params (LaunchVelocity :type Vector))
  (bind _outpathpositions (Class|GameplayStatics|BlueprintPredictProjectilePathbyObjectType (+ (Transformation|GetActorLocation) "0.000000,0.000000,100.000000") LaunchVelocity true 2.0 (Utilities|Array|MakeArray "ObjectTypeQuery1") false 0 "None" 0.0 15.0 2e+01))
  (CallFunction|CreateArkfromPossition _outpathpositions))

(fn CreateArkfromPossition
  (params (Possitions :type Array%20of%20Vectors))
  (for (_array_element _array_index) Possitions
    (if (!= _array_index 0)
      (bind _returnvalue (AddComponent|AddArrowComponent true (Utilities|MakeTransform _array_element (Utilities|Array|Get(acopy) Possitions (+ _array_index -1)))))
      (Variables|/Script/Engine.ArrowComponent|SetArrowSize _returnvalue 0.5))))