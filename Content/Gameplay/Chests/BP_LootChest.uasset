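; Interactable loot chest that opens, closes, can be locked, and drops its loot only once.
; An overlap box registers it in the actor's interaction queue and toggles a tooltip, while interaction acts on a Closed/Opened/Locked/InAction state machine.
; OpenTimeline, rate-scaled to AnimDuration, is meant to rotate the lid pivot.
; Lock and drop-loot components handle those jobs: unlocking auto-opens the chest, and opening triggers the drop as the animation starts.
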(event OnComponentBeginOverlap(IntteractBox)
  (params (OverlappedComponent :type Primitive%20Component%20Object%20Reference) (OtherActor :type Actor%20Object%20Reference) (OtherComp :type Primitive%20Component%20Object%20Reference) (OtherBodyIndex :type Integer) (bFromSweep :type Boolean) (SweepResult :type Hit%20Result%20Structure%20%28by%20ref%29))
  (CallFunction|AddtoInteractionQueue self OtherActor)
  (if (Utilities|Enum|Equal(Enum) (Variables|Default|GetCurrentState) "NewEnumerator1")
    (Rendering|SetVisibility (Variables|Default|Get%20TooltipWidget) true false)))

(event OnComponentEndOverlap(IntteractBox)
  (params (OverlappedComponent :type Primitive%20Component%20Object%20Reference) (OtherActor :type Actor%20Object%20Reference) (OtherComp :type Primitive%20Component%20Object%20Reference) (OtherBodyIndex :type Integer))
  (CallFunction|RemovefromInteractionQueue self OtherActor)
  (Rendering|SetVisibility (Variables|Default|Get%20TooltipWidget) false false))

(event EventTick
  (params (DeltaSeconds :type Float%20%28single-precision%29)))

(event EventBeginPlay
  (Components|Timeline|SetPlayRate (Variables|Default|GetOpenTimeline) (Math|Float|SafeDivide (Components|Timeline|GetTimelineLength (Variables|Default|GetOpenTimeline)) (Variables|Default|GetAnimDuration))))

(fn ConstructionScript
  (Variables|Default|SetInitialState (select (Utilities|Enum|Equal(Enum) (Variables|Default|GetInitialState) "NewEnumerator3") "NewEnumerator1" (Variables|Default|GetInitialState)))
  (bind _output_get (Variables|Default|SetCurrentState (Variables|Default|GetInitialState)))
  (CallFunction|AnimationOpen (Utilities|Select :Index _output_get :NewEnumerator0 1.0 :NewEnumerator1 0.0 :NewEnumerator2 0.0 :NewEnumerator3 0.0))
  (Variables|/Game/Components/BPAC_Lock.BPAC_Lock_C|SetIsLocked (Variables|Default|GetBPAC_Lock) (Utilities|Enum|Equal(Enum) (Variables|Default|GetCurrentState) "NewEnumerator2")))

(fn Close
  (Utilities|SwitchCurrentState
    (:Opened
      (Variables|Default|SetCurrentState "NewEnumerator3"))
    (:Closed
      (return false))
    (:Locked
      (return false))
    (:InAction
      (Utilities|SwitchTargetState
        (:Opened
          _)
        (:Closed
          (return false))
        (:Locked
          (return false))
        (:InAction
          (return false)))))
  (Variables|Default|SetTargetState "NewEnumerator1")
  (Components|Timeline|ReversefromEnd (Variables|Default|GetOpenTimeline))
  (return true))

(fn Open
  (Utilities|SwitchCurrentState
    (:Opened
      (return false))
    (:Closed
      (Variables|Default|SetCurrentState "NewEnumerator3"))
    (:Locked
      (return false))
    (:InAction
      (Utilities|SwitchTargetState
        (:Opened
          (return false))
        (:Closed
          _)
        (:Locked
          (return false))
        (:InAction
          (return false)))))
  (Variables|Default|SetTargetState "NewEnumerator0")
  (Components|Timeline|PlayfromStart (Variables|Default|GetOpenTimeline))
  (bind _success (CallFunction|DropLoot))
  (return _success))

(fn AnimationOpen
  (params (AnimProgress :type Float%20%28double-precision%29))
  (Transformation|SetRelativeRotation (Variables|Default|GetRotator) (Math|Rotator|MakeRotator (* (Variables|Default|GetMaxOpenAngle) AnimProgress) 0.0 0.0) false false))

(fn DropLoot
  (if (not (Variables|/Game/Components/BPAC_DropLoot.BPAC_DropLoot_C|GetIsDroped (Variables|Default|GetBPAC_DropLoot)))
    (Default|DropLoot (Variables|Default|GetBPAC_DropLoot))
    (bind _success (Default|SetIsDropped (Variables|Default|GetBPAC_DropLoot)))
    (return _success)
    (else
      (return false))))

(fn SetIsLocked
  (params (OtherActor :type Actor%20Object%20Reference) (IsLocked :type Boolean))
  (if IsLocked
    (if (Utilities|Enum|Equal(Enum) (Variables|Default|GetCurrentState) "NewEnumerator1")
      (bind _success (Default|Lock (Variables|Default|GetBPAC_Lock) OtherActor))
      (if _success
        (Variables|Default|SetCurrentState "NewEnumerator2")
        (return true)
        (else
          (return false)))
      (else
        (return false)))
    (elif (Utilities|Enum|Equal(Enum) (Variables|Default|GetCurrentState) "NewEnumerator2")
      (bind _success_2 (Default|Unlock (Variables|Default|GetBPAC_Lock) OtherActor))
      (if _success_2
        (Variables|Default|SetCurrentState "NewEnumerator1")
        (CallFunction|Open)
        (return true)
        (else
          (return false)))
      (else
        (return false)))))

(fn InteractionInterface
  (params (Interactor :type Actor%20Object%20Reference))
  (Utilities|SwitchCurrentState
    (:Opened
      (CallFunction|Close)
      (Rendering|SetVisibility (Variables|Default|Get%20TooltipWidget) true false)
      (return true))
    (:Closed
      (CallFunction|Open)
      (Rendering|SetVisibility (Variables|Default|Get%20TooltipWidget) false false)
      (return true))
    (:Locked
      (bind _success (CallFunction|SetIsLocked Interactor false))
      (return _success))
    (:InAction
      (return false))))