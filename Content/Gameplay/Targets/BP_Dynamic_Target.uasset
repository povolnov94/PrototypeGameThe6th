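; BP_Dynamic_Target is a moving target that shuttles endlessly between its spawn point and an offset set by the MovingRange variables.
; BeginPlay caches both endpoints, then a timeline lerps the actor to the end point.
; A second timeline, played in reverse, brings it back and restarts the first, forming a loop without Tick.
; The endpoints come from world location but are applied as relative location.
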(event EventBeginPlay
  (bind _returnvalue (Transformation|GetActorLocation))
  (Variables|Default|SetStartPoint (Math|Vector|MakeVector (.x _returnvalue) (.y _returnvalue) (.z _returnvalue)))
  (Variables|Default|SetEndPoint (Math|Vector|MakeVector (+ (.X (Math|Vector|BreakVector (Variables|Default|GetStartPoint))) (Variables|Default|GetMovingRangeX)) (+ (.Y (Math|Vector|BreakVector (Variables|Default|GetStartPoint))) (Variables|Default|GetMovingRangeY)) (+ (.Z (Math|Vector|BreakVector (Variables|Default|GetStartPoint))) (Variables|Default|GetMovingRangeZ))))
  (bind _move (Timeline|MoveDynamicTartget PlayFromStart)
    (:Update
      (Transformation|SetActorRelativeLocation (Math|Vector|Lerp(Vector) (Variables|Default|GetStartPoint) (Variables|Default|GetEndPoint) _move)))
    (:Finished
      (bind _move_2 (Timeline|Timeline ReverseFromEnd)
        (:Update
          (Transformation|SetActorRelativeLocation (Math|Vector|Lerp(Vector) (Variables|Default|GetStartPoint) (Variables|Default|GetEndPoint) _move_2)))
        (:Finished
          (Timeline|MoveDynamicTartget PlayFromStart))))))

(event EventTick
  (params (DeltaSeconds :type Float%20%28single-precision%29))
  (|CallParentFunction DeltaSeconds) ; This node is disabled and will not be called.\nDrag off pins to build functionality.
)

(fn ConstructionScript
  (|CallParentFunction))