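; Flame trap that bursts Niagara fire and periodically damages the player who enters its box trigger.
; Box overlap starts a looping timer that, gated by DoOnce, activates the flames after a short delay.
; If the player is inside the sphere, a damage timer runs until burst end, then DoOnce resets; otherwise the gate stays closed.
; Any actor leaving the box clears both timers and stops the flames.
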(event OnComponentBeginOverlap(BoxCollision)
  (params (OverlappedComponent :type Primitive%20Component%20Object%20Reference) (OtherActor :type Actor%20Object%20Reference) (OtherComp :type Primitive%20Component%20Object%20Reference) (OtherBodyIndex :type Integer) (bFromSweep :type Boolean) (SweepResult :type Hit%20Result%20Structure%20%28by%20ref%29))
  (bind _output_get (Variables|Default|SetOverlappedActor OtherActor))
  (if (== _output_get (Game|GetPlayerCharacter 0))
    (if (Utilities|Time|IsTimerActivebyHandle (Variables|Default|GetTrapTimer))
      (Utilities|Time|ClearandInvalidateTimerbyHandle (Variables|Default|GetTrapTimer))
      (Components|Activation|Deactivate (Variables|Default|GetNiagara))
      (Utilities|Time|ClearandInvalidateTimerbyHandle (Variables|Default|GetDamageTimer)))
    (bind _returnvalue (Utilities|Time|SetTimerbyEvent (delegate Custom|CustomEvent) 0.5 true))
    (Variables|Default|SetTrapTimer _returnvalue)))

(event OnComponentEndOverlap(BoxCollision)
  (params (OverlappedComponent :type Primitive%20Component%20Object%20Reference) (OtherActor :type Actor%20Object%20Reference) (OtherComp :type Primitive%20Component%20Object%20Reference) (OtherBodyIndex :type Integer))
  (Utilities|Time|ClearandInvalidateTimerbyHandle (Variables|Default|GetTrapTimer))
  (Components|Activation|Deactivate (Variables|Default|GetNiagara))
  (Utilities|Time|ClearandInvalidateTimerbyHandle (Variables|Default|GetDamageTimer)))

(event Custom|ApplyDamage
  (Game|Damage|ApplyDamage (Variables|Default|GetOverlappedActor) (Variables|Default|GetAmount) 0 0))

(event Custom|CustomEvent
  (Utilities|FlowControl|DoOnce false :!label _label
    (:Completed
      (Utilities|FlowControl|Delay 0.5)
      (Components|Activation|Activate (Variables|Default|GetNiagara) false)
      (if (Collision|IsOverlappingActor (Variables|Default|GetSphere) (Variables|Default|GetOverlappedActor) :!class /Script/Engine.PrimitiveComponent)
        (bind _returnvalue (Utilities|Time|SetTimerbyEvent (delegate Custom|ApplyDamage) 0.5 true))
        (Variables|Default|SetDamageTimer _returnvalue)
        (Utilities|FlowControl|Delay 1.5)
        (Components|Activation|Deactivate (Variables|Default|GetNiagara))
        (Utilities|Time|ClearandInvalidateTimerbyHandle (Variables|Default|GetDamageTimer))
        (goto _label Reset)))))

(fn ConstructionScript)