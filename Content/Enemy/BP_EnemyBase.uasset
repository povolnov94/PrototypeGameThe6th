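; Base enemy character that takes damage, attacks and dies through action components, with a health bar widget bound to its health component.
; Damage lowers health, then either alerts the AI controller that the player attacked or runs a one-time death action and fires OnKilled.
; Attacks start the attack action and attach a Niagara blade trail sized from two sockets.
; It also clears player sight when the player dies and draws patrol state each tick for debugging.
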(event EventTick
  (params (DeltaSeconds :type Float%20%28single-precision%29))
  (Rendering|Debug|DrawDebugString (+ (Transformation|GetWorldLocation (Variables|Collision|GetCapsuleComponent)) "0.000000,0.000000,20.000000") (Utilities|String|ToString(Text) (Utilities|Text|FormatText "{CurrentPatrolState} " (Utilities|String|EnumtoString (Variables|/Game/Components/BPAC_AIPatrolling.BPAC_AIPatrolling_C|GetPatrolState (Variables|Default|GetBPAC_AIManager))))) 0 "(R=0.000000,G=0.149960,B=0.122139,A=1.000000)"))

(event EventBeginPlay
  (EventDispatchers|BindEventtoOnTakeAnyDamage (EventDispatchers|CreateEvent :!event ApplyDamage))
  (bind _aswbp_enemy_health_bar (Utilities|Casting|CastToWBP_EnemyHealthBar (UserInterface|GetUserWidgetObject (Variables|Default|GetWidget))))
  (Default|SetUpWidget _aswbp_enemy_health_bar (Variables|Default|GetHealthComponent)))

(fn ConstructionScript)

(fn ApplyDamage
  (params (DamagedActor :type Actor%20Object%20Reference) (Damage :type Float%20%28single-precision%29) (DamageType :type Damage%20Type%20Object%20Reference) (InstigatedBy :type Controller%20Object%20Reference) (DamageCauser :type Actor%20Object%20Reference))
  (Default|DecreaseValue (Variables|Default|GetHealthComponent) Damage)
  (if (> (Default|GetCurValue (Variables|Default|GetHealthComponent)) 0.0)
    (bind _asbp_enemy_aicontroller (Utilities|Casting|CastToBP_EnemyAIController (AI|GetAIController self)))
    (Default|AttackedbyPlayer _asbp_enemy_aicontroller)
    (else
      (CallFunction|StartDeath))))

(fn StartDeath
  (if (not (Variables|Default|GetIsDead))
    (Default|StartAction (Variables|Default|GetBPAC_DeathAction))
    (Default|CallOnKilled)
    (Variables|Default|SetIsDead true)))

(fn AttackPlayer
  (params (AttackingActor :type Actor%20Object%20Reference))
  (bind _skeleton_blade (Variables|Default|GetSkeleton_Blade))
  (bind _skeleton_blade_2 (Variables|Default|GetSkeleton_Blade))
  (bind _returnvalue (Transformation|GetSocketLocation _skeleton_blade "Trail_Top"))
  (bind _returnvalue_2 (Transformation|GetSocketLocation _skeleton_blade "Trail_Bottom"))
  (bind _returnvalue_3 (- _returnvalue _returnvalue_2))
  (Default|StartAction (Variables|Default|GetBPAC_AttackAction) AttackingActor)
  (bind _returnvalue_4 (Niagara|SpawnSystemAttached "/Game/Art/FVX/NS_Trail.NS_Trail" (Variables|Default|GetSkeleton_Blade) "None" (/ (+ (Transformation|GetSocketLocation _skeleton_blade_2 "Trail_Top") (Transformation|GetSocketLocation _skeleton_blade_2 "Trail_Bottom")) 2.0) (Math|Rotator|MakeRotfromZ _returnvalue_3) "KeepWorldPosition" false))
  (Effects|Components|ParticleSystem|SetFloatParameter _returnvalue_4 "TrailWidth" (Math|Vector|VectorLength _returnvalue_3)))

(fn CheckIsTargetDead
  (if (<= (Default|GetCurValue (Actor|GetComponentbyClass (Game|GetPlayerCharacter 0) "/Game/Components/BPAC_Health.BPAC_Health_C")) 0.0)
    (AI|Components|Blackboard|SetValueasBool (AI|GetBlackboard 0) (Utilities|Name|MakeLiteralName "CanSeePlayer") false)
    (Variables|Default|SetIsAttacking false)
    (return true)
    (else
      (return false))))

(fn InteractionInterface
  (params (Interactor :type Actor%20Object%20Reference))
  (return true))