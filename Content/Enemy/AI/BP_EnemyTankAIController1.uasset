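; AI controller for the tank enemy that runs its behavior tree after a short startup delay.
; Perception events write target, visibility and last-seen location to the blackboard, while an AI state component switches between chasing and looking for the player.
; Being attacked stops movement, focuses the current target and enters a timed blocking state before resuming the chase.
; The memory-timeout path back to patrolling is unconnected.
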(event OnTargetPerceptionUpdated(AIPerception)
  (params (Actor :type Actor%20Object%20Reference) (Stimulus :type AI%20Stimulus%20Structure))
  (Variables|Default|SetTargetActor Actor)
  (if (>= (Utilities|Array|FindItem (Variables|/Script/Engine.Actor|GetTags (Variables|Default|GetTargetActor)) (Variables|Default|GetEnemyTag)) 0)
    (if (Utilities|Struct|BreakAIStimulus Stimulus)
      (CallFunction|FollowNewActorTarget (Variables|Default|GetTargetActor))
      (AI|Components|Blackboard|SetValueasBool (AI|GetBlackboard 0) (Utilities|Name|MakeLiteralName "CanSeePlayer") true)
      (else
        (AI|Components|Blackboard|SetValueasBool (AI|GetBlackboard 0) (Utilities|Name|MakeLiteralName "CanSeePlayer") false)
        (CallFunction|LookingforPlayer)))))

(event OnPerceptionUpdated(AIPerception)
  (params (UpdatedActors :type Array%20of%20Actor%20Object%20References))
  (if (Utilities|Array|ContainsItem UpdatedActors (Game|GetPlayerCharacter 0))
    (AI|Components|Blackboard|SetValueasObject (AI|GetBlackboard 0) (Variables|Default|GetChasingTargetKey) (Game|GetPlayerCharacter 0))
    (AI|Components|Blackboard|SetValueasVector (AI|GetBlackboard 0) (Utilities|Name|MakeLiteralName "LastTargetPoint") (Transformation|GetActorLocation (Game|GetPlayerCharacter 0)))))

(event EventBeginPlay
  (Utilities|FlowControl|Delay 3.0)
  (AI|RunBehaviorTree "/Game/Enemy/AI/BT_EnemyTankAI.BT_EnemyTankAI")
  (Default|SetLookingforPlayerState (Variables|Default|GetBPAC_AIState)))

(event EventTick
  (params (DeltaSeconds :type Float%20%28single-precision%29)))

(fn ConstructionScript)

(fn FollowNewActorTarget
  (params (FollowTargetActor :type Actor%20Object%20Reference))
  (Utilities|Time|ClearandInvalidateTimerbyHandle (Variables|Default|GetMemoryTimer))
  (AI|Components|Blackboard|SetValueasObject (AI|GetBlackboard 0) (Variables|Default|GetChasingTargetKey) FollowTargetActor)
  (if (Utilities|Enum|NotEqual(Enum) (Variables|/Game/Components/BPAC_AIStateMachine.BPAC_AIStateMachine_C|GetState (Variables|Default|GetBPAC_AIState)) "NewEnumerator3")
    (Default|SetChasingState (Variables|Default|GetBPAC_AIState))
    (return)))

(fn LookingforPlayer
  (Default|SetLookingforPlayerState (Variables|Default|GetBPAC_AIState)))

(fn AttackedbyPlayer
  (AI|Navigation|StopMovement)
  (AI|SetFocus (Variables|Default|GetTargetActor))
  (CallFunction|FollowNewActorTarget (Variables|Default|GetTargetActor))
  (AI|Components|Blackboard|SetValueasBool (AI|GetBlackboard 0) (Utilities|Name|MakeLiteralName "CanSeePlayer") true)
  (Default|SetBlockingState (Variables|Default|GetBPAC_AIState))
  (AI|Components|Blackboard|SetValueasBool (AI|GetBlackboard 0) (Utilities|Name|MakeLiteralName "IsBlocking") true)
  (Utilities|Time|SetTimerbyEvent (EventDispatchers|CreateEvent :!event BPEnemyTankAIControllerAutoGenFunc) 3.5))

(fn ClearAIMemory
  (AI|Components|Blackboard|SetValueasObject (AI|GetBlackboard 0) (Variables|Default|GetChasingTargetKey) (Variables|Default|GetTargetActor))
  (Default|SetPatrollingState (Variables|Default|GetBPAC_AIState))
  (return))

(fn BPEnemyTankAIControllerAutoGenFunc
  (AI|Components|Blackboard|SetValueasBool (AI|GetBlackboard 0) (Utilities|Name|MakeLiteralName "IsBlocking") false)
  (Default|SetChasingState (Variables|Default|GetBPAC_AIState))
  (AI|ClearFocus))