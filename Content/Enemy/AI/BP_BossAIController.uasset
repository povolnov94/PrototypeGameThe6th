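; AI controller for a boss enemy that runs the BT_BossAI behavior tree on activation and tracks targets through perception.
; Perception updates write chase target, CanSeePlayer and, for the player, last known location to the Blackboard.
; AttackedByPlayer forces the player as visible target.
; State changes and the memory-clearing timer are disconnected, so losing sight only clears CanSeePlayer.
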(event OnTargetPerceptionUpdated(AIPerception)
  (params (Actor :type Actor%20Object%20Reference) (Stimulus :type AI%20Stimulus%20Structure))
  (if (Variables|Default|GetIsBTActivated)
    (Variables|Default|SetTargetActor Actor)
    (if (>= (Utilities|Array|FindItem (Variables|/Script/Engine.Actor|GetTags (Variables|Default|GetTargetActor)) (Variables|Default|GetEnemyTag)) 0)
      (if (Utilities|Struct|BreakAIStimulus Stimulus)
        (CallFunction|FollowNewActorTarget (Variables|Default|GetTargetActor))
        (AI|Components|Blackboard|SetValueasBool (AI|GetBlackboard 0) (Utilities|Name|MakeLiteralName "CanSeePlayer") true)
        (else
          (AI|Components|Blackboard|SetValueasBool (AI|GetBlackboard 0) (Utilities|Name|MakeLiteralName "CanSeePlayer") false)
          (CallFunction|LookingforPlayer))))))

(event OnPerceptionUpdated(AIPerception)
  (params (UpdatedActors :type Array%20of%20Actor%20Object%20References))
  (if (Variables|Default|GetIsBTActivated)
    (if (Utilities|Array|ContainsItem UpdatedActors (Game|GetPlayerCharacter 0))
      (AI|Components|Blackboard|SetValueasObject (AI|GetBlackboard 0) (Variables|Default|GetChasingTargetKey) (Game|GetPlayerCharacter 0))
      (AI|Components|Blackboard|SetValueasVector (AI|GetBlackboard 0) (Utilities|Name|MakeLiteralName "LastTargetPoint") (Transformation|GetActorLocation (Game|GetPlayerCharacter 0))))))

(event Custom|Activate
  (AI|RunBehaviorTree "/Game/Enemy/AI/BT_BossAI.BT_BossAI")
  (Default|CallOnActivated)
  (Variables|Default|SetIsBTActivated true))

(event EventTick
  (params (DeltaSeconds :type Float%20%28single-precision%29)))

(fn ConstructionScript)

(fn FollowNewActorTarget
  (params (FollowTargetActor :type Actor%20Object%20Reference))
  (Utilities|Time|ClearandInvalidateTimerbyHandle (Variables|Default|GetMemoryTimer))
  (AI|Components|Blackboard|SetValueasObject (AI|GetBlackboard 0) (Variables|Default|GetChasingTargetKey) FollowTargetActor))

(fn LookingforPlayer)

(fn AttackedbyPlayer
  (CallFunction|FollowNewActorTarget (Game|GetPlayerCharacter 0))
  (AI|Components|Blackboard|SetValueasBool (AI|GetBlackboard 0) (Utilities|Name|MakeLiteralName "CanSeePlayer") true))

(fn ClearAIMemory
  (AI|Components|Blackboard|SetValueasObject (AI|GetBlackboard 0) (Variables|Default|GetChasingTargetKey) 0))