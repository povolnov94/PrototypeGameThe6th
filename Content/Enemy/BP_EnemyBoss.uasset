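; Boss enemy character that stays hidden until activated, then plays a spawn montage and shows a health bar.
; Damage outside its dissolve-material shield updates blackboard HP; health thresholds trigger enemy spawners, then move attack points and signal the AI state machine's shield phase.
; It offers fireball, knockback meteor and skull-spawner actions, with a zero-skull check starting phase three.
; Death drops loot, spawns explosions and destroys the actor.
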(event OnSeePawn(PawnSensing)
  (params (Pawn :type Pawn%20Object%20Reference))
  (Utilities|Casting|CastToBP_ThirdPersonCharacter Pawn)
  (Transformation|SetActorRotation (Math|Rotator|FindLookatRotation (Transformation|GetActorLocation) (Transformation|GetActorLocation Pawn))))

(event Custom|DeactivateShield
  (Rendering|Material|SetScalarParameterValue (Variables|Default|GetShieldMaterial) "Destory" 1.0 :!class /Script/Engine.MaterialInstanceDynamic)
  (bind _newtrack_0 (Timeline|Timeline_0 PlayFromStart)
    (:Update
      (Rendering|Material|SetScalarParameterValue (Variables|Default|GetShieldMaterial) "TimeSpeed" _newtrack_0 :!class /Script/Engine.MaterialInstanceDynamic)
      (Utilities|FlowControl|DoOnce false
        (:Completed
          (bind _newtrack_0_2 (Timeline|Timeline_1 ReverseFromEnd)
            (:Update
              (Rendering|Material|SetScalarParameterValue (Variables|Default|GetShieldMaterial) "DissolveAmount" _newtrack_0_2 :!class /Script/Engine.MaterialInstanceDynamic)
              (Utilities|FlowControl|Delay 1.0)
              (Rendering|SetVisibility (Variables|Default|GetSphere) false false)
              (Variables|Default|SetIsShieldEnable false))))))))

(event Custom|MeteorStrike
  (bind _returnvalue (Game|GetPlayerCharacter 0))
  (bind _returnvalue_2 (Game|SpawnActorfromClass "/Game/Weapons/MagickSpells/BP_AOEMeteorStrike.BP_AOEMeteorStrike_C" (Math|Transform|MakeTransform (Transformation|GetActorLocation _returnvalue) (Transformation|GetActorRotation _returnvalue) "1.000000,1.000000,1.000000") "Undefined" "MultiplyWithRoot" 0 1.9 _returnvalue false true false 5.0 0))
  (EventDispatchers|AssignOnAOEOverlapActor _returnvalue_2 (delegate Custom|PushBackPlayer)))

(event Custom|PushBackPlayer
  (params (Actor :type Actor%20Object%20Reference))
  (bind _returnvalue (Game|GetPlayerCharacter 0))
  (if (== Actor _returnvalue)
    (Character|LaunchCharacter _returnvalue "500.000000,500.000000,500.000000" true true)
    (Game|Damage|ApplyDamage Actor 2e+01 0 0)))

(event Custom|ActivateHPWidget
  (Rendering|SetVisibility (Variables|Collision|GetCapsuleComponent) true true)
  (Rendering|SetVisibility (Variables|Default|GetSphere) false false)
  (Animation|PlayAnimMontage "/Game/Assets/NEWSKELETONS/AM_BossSpawn.AM_BossSpawn" 1.0 "None")
  (bind _returnvalue (UserInterface|CreateWidget "/Game/Widgets/WBP_BossEnemyHealthBar.WBP_BossEnemyHealthBar_C"))
  (Variables|Default|SetHPWidget _returnvalue)
  (Default|SetUpWidget (Variables|Default|GetHPWidget) (Variables|Default|GetHealthComponent))
  (UserInterface|Viewport|AddtoViewport (Variables|Default|GetHPWidget) 0))

(event Custom|ActivateShield
  (bind _sphere (Variables|Default|GetSphere))
  (if (not (Variables|Default|GetIsShieldMICreated))
    (bind _returnvalue (Rendering|Material|CreateDynamicMaterialInstance _sphere 0 (Rendering|Material|GetMaterial _sphere 0) "None" :!class /Script/Engine.PrimitiveComponent))
    (Variables|Default|SetShieldMaterial _returnvalue)
    (Variables|Default|SetIsShieldMICreated true))
  (Rendering|SetVisibility (Variables|Default|GetSphere) true false)
  (bind _returnvalue_2 (Animation|PlayAnimMontage "/Game/Enemy/Animation/AM_ShieldCast.AM_ShieldCast" 1.0 "None"))
  (Utilities|FlowControl|Delay _returnvalue_2)
  (Variables|Default|SetIsShieldEnable true)
  (bind _newtrack_0 (Timeline|Timeline PlayFromStart)
    (:Update
      (Rendering|Material|SetScalarParameterValue (Variables|Default|GetShieldMaterial) "DissolveAmount" _newtrack_0 :!class /Script/Engine.MaterialInstanceDynamic)
      (Rendering|Material|SetScalarParameterValue (Variables|Default|GetShieldMaterial) "Destory" 0.0 :!class /Script/Engine.MaterialInstanceDynamic)
      (Utilities|FlowControl|DoOnce false) ; enters at Reset
    )))

(event EventBeginPlay
  (Rendering|SetVisibility (Variables|Collision|GetCapsuleComponent) false true)
  (EventDispatchers|BindEventtoOnTakeAnyDamage (EventDispatchers|CreateEvent :!event ApplyDamage))
  (bind _asbp_boss_aicontroller (Utilities|Casting|CastToBP_BossAIController (AI|GetAIController self)))
  (EventDispatchers|BindEventtoOnActivated _asbp_boss_aicontroller (EventDispatchers|CreateEvent :!event SetBlackboardValues)))

(fn ConstructionScript)

(fn ApplyDamage
  (params (DamagedActor :type Actor%20Object%20Reference) (Damage :type Float%20%28single-precision%29) (DamageType :type Damage%20Type%20Object%20Reference) (InstigatedBy :type Controller%20Object%20Reference) (DamageCauser :type Actor%20Object%20Reference))
  (bind _returnvalue (Pawn|GetController))
  (bind _returnvalue_2 (Actor|GetComponentbyClass _returnvalue "/Game/Components/BPAC_BossAIStateMachine.BPAC_BossAIStateMachine_C"))
  (if (not (Variables|Default|GetIsShieldEnable))
    (Default|DecreaseValue (Variables|Default|GetHealthComponent) Damage)
    (Game|SpawnActorfromClass "/Game/Widgets/DMGAmount/BP_DmgAmount.BP_DmgAmount_C" (Transformation|GetWorldTransform (Variables|Default|GetSphere)) "Undefined" "MultiplyWithRoot" 0 Damage 0)
    (AI|Components|Blackboard|SetValueasFloat (AI|GetBlackboard 0) (Utilities|Name|MakeLiteralName "BossHP") (Default|GetCurValue (Variables|Default|GetHealthComponent)))
    (if (> (Default|GetCurValue (Variables|Default|GetHealthComponent)) 0.0)
      (if (and (< (Default|GetCurValue (Variables|Default|GetHealthComponent)) 444.0) (> (Default|GetCurValue (Variables|Default|GetHealthComponent)) 222.0))
        (Utilities|FlowControl|DoOnce false
          (:Completed
            (Variables|Default|SetAttackPoint 1)
            (CallFunction|ActivateEnemySpawners)))
        (elif (<= (Default|GetCurValue (Variables|Default|GetHealthComponent)) 222.0)
          (Utilities|FlowControl|DoOnce false
            (:Completed
              (AI|Components|Blackboard|SetValueasBool (AI|GetBlackboard 0) (Utilities|Name|MakeLiteralName "IsNewAttackPointSet") false)
              (if (Utilities|Enum|Equal(Enum) (Variables|/Game/Components/BPAC_BossAIStateMachine.BPAC_BossAIStateMachine_C|GetState _returnvalue_2) "NewEnumerator1")
                (Default|SetPhase2Shield _returnvalue_2)
                (Variables|Default|SetAttackPoint 2)
                (CallFunction|SetAttackPoint))))))
      (else
        (CallFunction|StartDeath)))))

(fn StartDeath
  (bind _returnvalue (Math|Random|RandomFloatinRange 1e+02 2.5e+02))
  (bind _returnvalue_2 (Math|Random|RandomFloatinRange 1e+02 2.5e+02))
  (bind _mesh (Variables|Character|GetMesh))
  (bind _mesh_2 (Variables|Character|GetMesh))
  (bind _mesh_3 (Variables|Character|GetMesh))
  (bind _returnvalue_3 (Transformation|GetWorldLocation _mesh))
  (bind _returnvalue_4 (Transformation|GetWorldLocation _mesh_3))
  (if (not (Variables|Default|GetIsDead))
    (Default|DropLoot (Variables|Default|GetBPAC_DropLoot))
    (Niagara|SpawnSystematLocation "/Game/Art/VFX/NS_SelfBombExplosion.NS_SelfBombExplosion" (Transformation|GetWorldLocation _mesh_2) (Transformation|GetWorldRotation _mesh_2))
    (Niagara|SpawnSystematLocation "/Game/Art/VFX/NS_SelfBombExplosion.NS_SelfBombExplosion" (Math|Vector|MakeVector (+ (.x _returnvalue_4) _returnvalue_2) (+ (.y _returnvalue_4) _returnvalue_2) (+ (.z _returnvalue_4) _returnvalue_2)))
    (Niagara|SpawnSystematLocation "/Game/Art/VFX/NS_SelfBombExplosion.NS_SelfBombExplosion" (Math|Vector|MakeVector (+ (.x _returnvalue_3) _returnvalue) (+ (.y _returnvalue_3) _returnvalue) (+ (.z _returnvalue_3) _returnvalue)))
    (Default|CallOnKilled)
    (Variables|Default|SetIsDead true)
    (Widget|RemovefromParent (Variables|Default|GetHPWidget))
    (Actor|DestroyActor)))

(fn AttackPlayer
  (params (AttackingActor :type Actor%20Object%20Reference))
  (Default|StartAction (Variables|Default|GetBPAC_AttackAction) AttackingActor))

(fn CheckIsTargetDead
  (if (<= (Default|GetCurValue (Actor|GetComponentbyClass (Game|GetPlayerCharacter 0) "/Game/Components/BPAC_Health.BPAC_Health_C")) 0.0)
    (AI|Components|Blackboard|SetValueasBool (AI|GetBlackboard 0) (Utilities|Name|MakeLiteralName "CanSeePlayer") false)
    (Variables|Default|SetIsAttacking false)
    (return true)
    (else
      (return false))))

(fn ShootFireballs
  (bind _mesh (Variables|Character|GetMesh))
  (bind _returnvalue (Transformation|GetWorldLocation _mesh))
  (bind (_outhit _returnvalue_2) (Collision|SphereTraceByChannel _returnvalue (+ _returnvalue (* (Math|Vector|GetForwardVector (Variables|Collision|GetCapsuleComponent)) (Variables|Default|GetAttackRange))) 1.5e+02 "TraceTypeQuery2" true (Utilities|Array|MakeArray self) "None" true "(R=1.000000,G=0.000000,B=0.000000,A=1.000000)" "(R=0.000000,G=1.000000,B=0.000000,A=1.000000)" 1.0))
  (if (Utilities|IsValid (.HitActor (Collision|BreakHitResult _outhit)))
    (LocalVariables|SetL_Direction (Math|Vector|Normalize (- (Math|Vector|SelectVector (.ImpactPoint (Collision|BreakHitResult _outhit)) (.TraceEnd (Collision|BreakHitResult _outhit)) _returnvalue_2) (Transformation|GetWorldLocation (Variables|Default|GetMuzzleFX)))))
    (Game|SpawnActorfromClass "/Game/Weapons/BaseClasses/BP_Fireball.BP_Fireball_C" (Transformation|GetWorldTransform (Variables|Default|GetMuzzleFX)) "AdjustIfPossibleButAlwaysSpawn" "MultiplyWithRoot" 0 (LocalVariables|GetL_Direction) 25 0)))

(fn SetAttackPoint
  (bind _output_get (Variables|Default|SetCurrentAttackPoint (Transformation|GetActorLocation (Utilities|Array|Get(acopy) (Variables|Default|GetPatrolPoints) (Variables|Default|GetAttackPoint)))))
  (AI|Components|Blackboard|SetValueasVector (AI|GetBlackboard 0) (Utilities|Name|MakeLiteralName "AttackPoint") _output_get))

(fn RotatetoPlayer
  (Transformation|SetActorRotation (Math|Rotator|FindLookatRotation (Transformation|GetActorLocation) (Transformation|GetActorLocation (Game|GetPlayerCharacter 0)))))

(fn ActivateSpawners
  (for _array_element (Variables|Default|GetSkullSpawners)
    (bind _asbp_skull_spawner (Utilities|Casting|CastToBP_SkullSpawner _array_element))
    (Default|Spawn _asbp_skull_spawner)
    (Variables|Default|SetCurrenAliveSkulls (+ (Variables|Default|GetCurrenAliveSkulls) 1.0))))

(fn CastMeteorStrike)

(fn CheckAliveSkulls
  (if (== (Variables|Default|GetCurrenAliveSkulls) 0.0)
    (Default|SetPhase3Attack (Actor|GetComponentbyClass (Pawn|GetController) "/Game/Components/BPAC_BossAIStateMachine.BPAC_BossAIStateMachine_C"))))

(fn SetBlackboardValues
  (AI|Components|Blackboard|SetValueasFloat (AI|GetBlackboard 0) (Utilities|Name|MakeLiteralName "BossHP") (Default|GetCurValue (Variables|Default|GetHealthComponent)))
  (CallFunction|SetAttackPoint))

(fn ActivateEnemySpawners
  (for _array_element (Variables|Default|GetEnemySpawners)
    (bind _asbp_enemy_spawner (Utilities|Casting|CastToBP_EnemySpawner _array_element))
    (Utilities|IsValid _asbp_enemy_spawner
      (:Is%20Valid
        (Default|SpawnEnemy _asbp_enemy_spawner)))))

(fn InteractionInterface
  (params (Interactor :type Actor%20Object%20Reference))
  (return true))