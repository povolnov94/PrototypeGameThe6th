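; Self-destructing "Bomber" enemy character that explodes to damage nearby players.
; Attacking freezes movement, plays a montage, reveals an indicator plane and starts a roughly three-second timer.
; Taking damage lowers health, spawns damage numbers and either alerts its AI controller or triggers death with loot and explosion VFX.
; The blast damages player characters overlapping its sphere, fires a radial impulse, reports the kill and destroys the actor.
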(event EventTick
  (params (DeltaSeconds :type Float%20%28single-precision%29)))

(event EventBeginPlay
  (EventDispatchers|BindEventtoOnTakeAnyDamage (EventDispatchers|CreateEvent :!event ApplyDamage))
  (bind _aswbp_enemy_health_bar (Utilities|Casting|CastToWBP_EnemyHealthBar (UserInterface|GetUserWidgetObject (Variables|Default|GetWidget))))
  (Default|SetEnemyName _aswbp_enemy_health_bar "Bomber")
  (Default|SetUpWidget _aswbp_enemy_health_bar (Variables|Default|GetHealthComponent)))

(fn ConstructionScript)

(fn ApplyDamage
  (params (DamagedActor :type Actor%20Object%20Reference) (Damage :type Float%20%28single-precision%29) (DamageType :type Damage%20Type%20Object%20Reference) (InstigatedBy :type Controller%20Object%20Reference) (DamageCauser :type Actor%20Object%20Reference))
  (Default|DecreaseValue (Variables|Default|GetHealthComponent) Damage)
  (Game|SpawnActorfromClass "/Game/Widgets/DMGAmount/BP_DmgAmount.BP_DmgAmount_C" (Transformation|GetActorTransform) "Undefined" "MultiplyWithRoot" 0 Damage 0)
  (if (> (Default|GetCurValue (Variables|Default|GetHealthComponent)) 0.0)
    (bind _asbp_enemy_self_bomb_aicontroller (Utilities|Casting|CastToBP_EnemySelfBombAIController (AI|GetAIController self)))
    (Default|AttackedbyPlayer _asbp_enemy_self_bomb_aicontroller)
    (else
      (Default|DropLoot (Variables|Default|GetBPAC_DropLoot))
      (CallFunction|StartDeath))))

(fn StartDeath
  (if (not (Variables|Default|GetIsDead))
    (Niagara|SpawnSystematLocation "/Game/Art/FVX/NS_SelfBombExplosion.NS_SelfBombExplosion" (Transformation|GetActorLocation) (Transformation|GetActorRotation))
    (Default|DropLoot (Variables|Default|GetBPAC_DropLoot))
    (CallFunction|EnemySelfBombAutoGenFunc)
    (Variables|Default|SetIsDead true)
    (Actor|DestroyActor)))

(fn AttackPlayer
  (params (AttackingActor :type Actor%20Object%20Reference))
  (Pawn|Components|CharacterMovement|DisableMovement (Variables|Character|GetCharacterMovement))
  (Animation|PlayAnimMontage "/Game/Enemy/AM_SelfTest.AM_SelfTest" 1.0 "None")
  (Rendering|SetVisibility (Variables|Default|GetPlane) true false)
  (Utilities|Time|SetTimerbyEvent (EventDispatchers|CreateEvent :!event BPEnemySelfBombAutoGenFunc) 3.07))

(fn CheckIsTargetDead
  (if (<= (Default|GetCurValue (Actor|GetComponentbyClass (Game|GetPlayerCharacter 0) "/Game/Components/BPAC_Health.BPAC_Health_C")) 0.0)
    (AI|Components|Blackboard|SetValueasBool (AI|GetBlackboard 0) (Utilities|Name|MakeLiteralName "CanSeePlayer") false)
    (Variables|Default|SetIsAttacking false)
    (return true)
    (else
      (return false))))

(fn BPEnemySelfBombAutoGenFunc
  (Variables|Default|SetIsAttacking true)
  (for _array_element (Collision|GetOverlappingActors (Variables|Default|GetSphere) "/Game/Characters/BP_ThirdPersonCharacter.BP_ThirdPersonCharacter_C" :!class /Script/Engine.PrimitiveComponent)
    (Utilities|IsValid (Actor|GetComponentbyClass _array_element "/Game/Components/BPAC_Health.BPAC_Health_C")
      (:Is%20Valid
        (Game|Damage|ApplyDamage _array_element 5e+01 0 self))))
  (Class|RadialForceComponent|FireImpulse (Variables|Default|GetRadialForce))
  (Default|CallOnKilled)
  (Actor|DestroyActor))

(fn TurnonSpeedUpVFX
  (Components|Activation|Activate (Variables|Default|GetNS_DashEffect) false))

(fn TurnOffSpeedUpVFX
  (Components|Activation|Deactivate (Variables|Default|GetNS_DashEffect)))

(fn InteractionInterface
  (params (Interactor :type Actor%20Object%20Reference))
  (return true))