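; Base enemy area-of-effect blast actor that adds visual and audio feedback to the parent class's Trigger.
; Trigger calls the parent, then spawns the Niagara BlastEffect attached to the root and plays BlastSound, which is gated on BlastEffect's validity.
; Without an effect, the actor destroys itself after a short delay.
; The SystemFinished destroy handler's binding is unconnected, so the effect's completion does not destroy the actor here.
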(event Custom|SystemFinished
  (params (PSystem :type Niagara%20Component%20Object%20Reference))
  (Actor|DestroyActor))

(event Custom|PlayBlastEffect
  (bind _blasteffect (Variables|Default|GetBlastEffect)
    (:then
      (bind _returnvalue (Niagara|SpawnSystemAttached _blasteffect (Variables|Default|GetDefaultSceneRoot) "None" "0, 0, 0" "0, 0, 0" "KeepRelativeOffset" true)))
    (:else
      (Utilities|FlowControl|Delay 0.2)
      (Actor|DestroyActor))))

(event Custom|PlayBlastSound
  (Variables|Default|GetBlastEffect
    (:then
      (Audio|PlaySoundatLocation (Variables|Default|GetBlastSound) (Transformation|GetActorLocation) "0, 0, 0" 1.0 1.0 0.0 0 0 0 0))
    (:else)))

(event EventBeginPlay
  (|CallParentFunction) ; This node is disabled and will not be called.\nDrag off pins to build functionality.
)

(event Collision|EventActorBeginOverlap
  (params (OtherActor :type Actor%20Object%20Reference)))

(event EventTick
  (params (DeltaSeconds :type Float%20%28single-precision%29)))

(event EventTrigger
  (|CallParentFunction)
  (CallFunction|PlayBlastEffect)
  (CallFunction|PlayBlastSound))

(fn ConstructionScript
  (|CallParentFunction))