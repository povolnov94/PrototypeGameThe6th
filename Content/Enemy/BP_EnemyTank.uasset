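; Shield-bearing tank enemy that blocks when hit, attacks with a block-attack montage and starts a death action at zero health.
; Damage feeds the health component, raises two block planes and alerts its AI controller; the first plane destroys any actor overlapping it.
; BeginPlay sets up the health bar and a toggleable Niagara spin trail sized from two shield sockets.
; Tick shows debug patrol, attack and block state.
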(event OnComponentBeginOverlap(Plane)
  (params (OverlappedComponent :type Primitive%20Component%20Object%20Reference) (OtherActor :type Actor%20Object%20Reference) (OtherComp :type Primitive%20Component%20Object%20Reference) (OtherBodyIndex :type Integer) (bFromSweep :type Boolean) (SweepResult :type Hit%20Result%20Structure%20%28by%20ref%29))
  (Actor|DestroyActor OtherActor))

(event EventTick
  (params (DeltaSeconds :type Float%20%28single-precision%29))
  (Rendering|Debug|DrawDebugString (+ (Transformation|GetWorldLocation (Variables|Collision|GetCapsuleComponent)) "0.000000,0.000000,20.000000") (Utilities|String|ToString(Text) (Utilities|Text|FormatText "{CurrentPatrolState} " (Utilities|String|EnumtoString (Variables|/Game/Components/BPAC_AIPatrolling.BPAC_AIPatrolling_C|GetPatrolState (Variables|Default|GetBPAC_AIManager))))) 0 "(R=0.000000,G=0.149960,B=0.122139,A=1.000000)")
  (Development|PrintString (Utilities|String|ToString(Text) (Utilities|Text|FormatText "{A} { B } " (Variables|Default|GetIsAttacking) (Variables|Default|GetIsBlocking))) true false "(R=0.000000,G=1.000000,B=0.012712,A=1.000000)" 0.0))

(event EventBeginPlay
  (bind _skeleton_shield_small_b (Variables|Default|GetSkeleton_Shield_Small_B))
  (bind _skeleton_shield_small_b_2 (Variables|Default|GetSkeleton_Shield_Small_B))
  (bind _returnvalue (Transformation|GetSocketLocation _skeleton_shield_small_b_2 "Trail_Top"))
  (bind _returnvalue_2 (Transformation|GetSocketLocation _skeleton_shield_small_b_2 "Trail_Bottom"))
  (bind _returnvalue_3 (- _returnvalue _returnvalue_2))
  (EventDispatchers|BindEventtoOnTakeAnyDamage (EventDispatchers|CreateEvent :!event ApplyDamage))
  (bind _aswbp_enemy_health_bar (Utilities|Casting|CastToWBP_EnemyHealthBar (UserInterface|GetUserWidgetObject (Variables|Default|GetWidget))))
  (Default|SetUpWidget _aswbp_enemy_health_bar (Variables|Default|GetHealthComponent))
  (bind _returnvalue_4 (Niagara|SpawnSystemAttached "/Game/Art/FVX/NS_Trail.NS_Trail" (Variables|Default|GetSkeleton_Shield_Small_B) "None" (/ (+ (Transformation|GetSocketLocation _skeleton_shield_small_b "Trail_Top") (Transformation|GetSocketLocation _skeleton_shield_small_b "Trail_Bottom")) 2.0) (Math|Rotator|MakeRotfromZ _returnvalue_3) "KeepWorldPosition" false false))
  (bind _output_get (Variables|Default|SetNS_Trail _returnvalue_4))
  (Effects|Components|ParticleSystem|SetFloatParameter _output_get "TrailWidth" (Math|Vector|VectorLength _returnvalue_3)))

(fn ConstructionScript)

(fn ApplyDamage
  (params (DamagedActor :type Actor%20Object%20Reference) (Damage :type Float%20%28single-precision%29) (DamageType :type Damage%20Type%20Object%20Reference) (InstigatedBy :type Controller%20Object%20Reference) (DamageCauser :type Actor%20Object%20Reference))
  (Default|DecreaseValue (Variables|Default|GetHealthComponent) Damage)
  (if (> (Default|GetCurValue (Variables|Default|GetHealthComponent)) 0.0)
    (Variables|Default|SetIsBlocking true)
    (Variables|Default|SetIsAttacking false)
    (CallFunction|ActivateBlock)
    (bind _asbp_enemy_tank_aicontroller (Utilities|Casting|CastToBP_EnemyTankAIController (AI|GetAIController self)))
    (Default|AttackedbyPlayer _asbp_enemy_tank_aicontroller)
    (else
      (CallFunction|StartDeath))))

(fn StartDeath
  (if (not (Variables|Default|GetIsDead))
    (Default|StartAction (Variables|Default|GetBPAC_DeathAction))
    (Default|CallOnKilled)
    (Variables|Default|SetIsDead true)))

(fn AttackPlayer
  (params (AttackingActor :type Actor%20Object%20Reference))
  (Animation|PlayAnimMontage "/Game/Enemy/AM_Block_Attack.AM_Block_Attack" 1.0 "None"))

(fn CheckIsTargetDead
  (if (<= (Default|GetCurValue (Actor|GetComponentbyClass (Game|GetPlayerCharacter 0) "/Game/Components/BPAC_Health.BPAC_Health_C")) 0.0)
    (AI|Components|Blackboard|SetValueasBool (AI|GetBlackboard 0) (Utilities|Name|MakeLiteralName "CanSeePlayer") false)
    (Variables|Default|SetIsAttacking false)
    (return true)
    (else
      (return false))))

(fn ClearFocus
  (AI|ClearFocus (AI|GetAIController self)))

(fn ActivateBlock
  (Rendering|SetVisibility (Variables|Default|GetPlane1) true false)
  (Collision|SetCollisionEnabled (Variables|Default|GetPlane1) "QueryAndPhysics"))

(fn DisableBlock
  (Rendering|SetVisibility (Variables|Default|GetPlane1) false false)
  (Collision|SetCollisionEnabled (Variables|Default|GetPlane1) "NoCollision"))

(fn ActivateSpinEffect
  (Components|Activation|Activate (Variables|Default|GetNS_Trail) false))

(fn DeactivateSpinEffect
  (Components|Activation|Deactivate (Variables|Default|GetNS_Trail)))

(fn InteractionInterface
  (params (Interactor :type Actor%20Object%20Reference))
  (return true))