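; BP_EnemyMinion is a melee enemy character with a spawn montage and a named health bar widget.
; Damage lowers its health component and spawns a damage-number actor, then either alerts the AI controller or triggers death, which drops loot and runs a death action.
; Attacks run through an action component and attach a Niagara trail sized from the blade's socket positions.
; A target check clears blackboard sight once the player is dead.
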(event EventTick
  (params (DeltaSeconds :type Float%20%28single-precision%29)))

(event EventBeginPlay
  (Animation|PlayAnimMontage (Utilities|Select :Index (Math|Random|RandomInteger 1) :Option%200 "/Game/Assets/NEWSKELETONS/AM_Spawn1.AM_Spawn1" :Option%201 "/Game/Assets/NEWSKELETONS/AM_Spawn2.AM_Spawn2") 1.0 "None")
  (EventDispatchers|BindEventtoOnTakeAnyDamage (EventDispatchers|CreateEvent :!event ApplyDamage))
  (bind _aswbp_enemy_health_bar (Utilities|Casting|CastToWBP_EnemyHealthBar (UserInterface|GetUserWidgetObject (Variables|Default|GetWidget))))
  (Default|SetEnemyName _aswbp_enemy_health_bar "Minion")
  (Default|SetUpWidget _aswbp_enemy_health_bar (Variables|Default|GetHealthComponent)))

(fn ConstructionScript)

(fn ApplyDamage
  (params (DamagedActor :type Actor%20Object%20Reference) (Damage :type Float%20%28single-precision%29) (DamageType :type Damage%20Type%20Object%20Reference) (InstigatedBy :type Controller%20Object%20Reference) (DamageCauser :type Actor%20Object%20Reference))
  (Default|DecreaseValue (Variables|Default|GetHealthComponent) Damage)
  (Game|SpawnActorfromClass "/Game/Widgets/DMGAmount/BP_DmgAmount.BP_DmgAmount_C" (Transformation|GetActorTransform) "Undefined" "MultiplyWithRoot" 0 Damage 0)
  (if (> (Default|GetCurValue (Variables|Default|GetHealthComponent)) 0.0)
    (bind _asbp_enemy_aicontroller (Utilities|Casting|CastToBP_EnemyAIController (AI|GetAIController self)))
    (Default|AttackedbyPlayer _asbp_enemy_aicontroller)
    (else
      (CallFunction|StartDeath))))

(fn StartDeath
  (if (not (Variables|Default|GetIsDead))
    (Default|DropLoot (Variables|Default|GetBPAC_DropLoot))
    (Default|StartAction (Variables|Default|GetBPAC_DeathAction))
    (Default|CallOnKilled)
    (Variables|Default|SetIsDead true)))

(fn AttackPlayer
  (params (AttackingActor :type Actor%20Object%20Reference))
  (bind _skeleton_blade (Variables|Default|GetSkeleton_Blade))
  (bind _skeleton_blade_2 (Variables|Default|GetSkeleton_Blade))
  (bind _returnvalue (Transformation|GetSocketLocation _skeleton_blade "Trail_Top"))
  (bind _returnvalue_2 (Transformation|GetSocketLocation _skeleton_blade "Trail_Bottom"))
  (bind _returnvalue_3 (- _returnvalue _returnvalue_2))
  (Default|StartAction (Variables|Default|GetBPAC_AttackAction) AttackingActor)
  (bind _returnvalue_4 (Niagara|SpawnSystemAttached "/Game/Art/VFX/NS_Trail.NS_Trail" (Variables|Default|GetSkeleton_Blade) "None" (/ (+ (Transformation|GetSocketLocation _skeleton_blade_2 "Trail_Top") (Transformation|GetSocketLocation _skeleton_blade_2 "Trail_Bottom")) 2.0) (Math|Rotator|MakeRotfromZ _returnvalue_3) "KeepWorldPosition" false))
  (Effects|Components|ParticleSystem|SetFloatParameter _returnvalue_4 "TrailWidth" (Math|Vector|VectorLength _returnvalue_3)))

(fn CheckIsTargetDead
  (if (<= (Default|GetCurValue (Actor|GetComponentbyClass (Game|GetPlayerCharacter 0) "/Game/Components/BPAC_Health.BPAC_Health_C")) 0.0)
    (AI|Components|Blackboard|SetValueasBool (AI|GetBlackboard 0) (Utilities|Name|MakeLiteralName "CanSeePlayer") false)
    (Variables|Default|SetIsAttacking false)
    (return true)
    (else
      (return false))))

(fn InteractionInterface
  (params (Interactor :type Actor%20Object%20Reference))
  (return true))