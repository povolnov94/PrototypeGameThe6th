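; Skull enemy that can be damaged and killed, and is counted by BP_EnemyBoss as one of its living skulls.
; AnyDamage lowers the BPACHealth component through TakeDamage, then spawns a BP_DmgAmount actor showing the hit at its transform.
; At zero health it decrements the count on the first boss found by GetAllActorsOfClass, calls CheckAliveSkulls and destroys itself.
; An OnSkullKilled dispatcher call and a cast-based boss update remain unconnected.
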(event Game|Damage|EventAnyDamage
  (params (Damage :type Float%20%28single-precision%29) (DamageType :type Damage%20Type%20Object%20Reference) (InstigatedBy :type Controller%20Object%20Reference) (DamageCauser :type Actor%20Object%20Reference))
  (CallFunction|TakeDamage Damage)
  (Game|SpawnActorfromClass "/Game/Widgets/DMGAmount/BP_DmgAmount.BP_DmgAmount_C" (Transformation|GetActorTransform) "Undefined" "MultiplyWithRoot" 0 Damage 0))

(event EventBeginPlay)

(fn ConstructionScript)

(fn TakeDamage
  (params (Amount :type Float%20%28double-precision%29))
  (Default|DecreaseValue (Variables|Default|GetBPAC_Health) Amount)
  (if (<= (Default|GetCurValue (Variables|Default|GetBPAC_Health)) 0.0)
    (bind _outactors (Actor|GetAllActorsOfClass "/Game/Enemy/BP_EnemyBoss.BP_EnemyBoss_C"))
    (Variables|/Game/Enemy/BP_EnemyBoss.BP_EnemyBoss_C|SetCurrenAliveSkulls (Utilities|Array|Get(acopy) _outactors) (- (Variables|/Game/Enemy/BP_EnemyBoss.BP_EnemyBoss_C|GetCurrenAliveSkulls (Utilities|Array|Get(acopy) _outactors)) 1.0))
    (Default|CheckAliveSkulls (Utilities|Array|Get(acopy) _outactors))
    (Actor|DestroyActor)))

(fn BPSkullEnemyAutoGenFunc
  (params (DestroyedActor :type Actor%20Object%20Reference)))