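; BP_PickupKeyBase is a base pickup that grants a key to the actor collecting it.
; Its ActivatePickupEffect looks up the BPAC_KeyChain component on the target actor and calls AddKey with the pickup's KeyClass.
; It returns the AddKey result, or false when the target has no key chain.
; The event graph and construction script add no logic beyond parent calls.
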(event EventBeginPlay
  (|CallParentFunction) ; This node is disabled and will not be called.\nDrag off pins to build functionality.
)

(event Collision|EventActorBeginOverlap
  (params (OtherActor :type Actor%20Object%20Reference))
  (|CallParentFunction OtherActor) ; This node is disabled and will not be called.\nDrag off pins to build functionality.
)

(event EventTick
  (params (DeltaSeconds :type Float%20%28single-precision%29))
  (|CallParentFunction DeltaSeconds) ; This node is disabled and will not be called.\nDrag off pins to build functionality.
)

(fn ConstructionScript
  (|CallParentFunction))

(fn ActivatePickupEffect
  (params (TargetActor :type Actor%20Object%20Reference))
  (bind _output_get (LocalVariables|SetL_KeyChain (Actor|GetComponentbyClass TargetActor "/Game/Components/BPAC_KeyChain.BPAC_KeyChain_C")))
  (Utilities|IsValid _output_get
    (:Is%20Valid
      (bind _success (Default|AddKey (LocalVariables|GetL_KeyChain) (Variables|Default|GetKeyClass)))
      (return _success))
    (:Is%20Not%20Valid
      (return false))))