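; Health pickup Blueprint that heals the actor it is activated on by its HealPower amount.
; ActivatePickupEffect finds the target's BPAC_Health component and increases its value without clamping to max, but only when health is not already equal to MaxValue.
; It returns the increase result, or false when the target is invalid, lacks the component or is at max health.
; The construction script only calls the parent.
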(fn ConstructionScript
  (|CallParentFunction))

(fn ActivatePickupEffect
  (params (TargetActor :type Actor%20Object%20Reference))
  (Utilities|IsValid TargetActor
    (:Is%20Valid
      (bind _output_get (LocalVariables|SetL_HealthComp (Actor|GetComponentbyClass TargetActor "/Game/Components/BPAC_Health.BPAC_Health_C")))
      (Utilities|IsValid _output_get
        (:Is%20Valid
          (if (not (== (Default|GetCurValue (LocalVariables|GetL_HealthComp)) (Variables|/Game/Components/BPAC_EntityResourse.BPAC_EntityResourse_C|GetMaxValue (LocalVariables|GetL_HealthComp))))
            (bind _success (Default|IncreaseValue (LocalVariables|GetL_HealthComp) (Variables|Default|GetHealPower) false))
            (return _success)
            (else
              (return false))))
        (:Is%20Not%20Valid
          (return false))))
    (:Is%20Not%20Valid
      (return false))))