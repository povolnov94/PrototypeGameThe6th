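; BP_Pickup_Common is a pickup actor that calls ActivatePickup when an actor overlaps its Box.
; The construction script gives the mesh dynamic materials and colors them and the glow particles by pickup Type: weapon, ammo, potion or bombs.
; When IsRotate is set, Tick runs FloatAndRotate, which eases the mesh up and down from its starting location with a ping-pong alpha while spinning it in yaw.
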(event OnComponentBeginOverlap(Box)
  (params (OverlappedComponent :type Primitive%20Component%20Object%20Reference) (OtherActor :type Actor%20Object%20Reference) (OtherComp :type Primitive%20Component%20Object%20Reference) (OtherBodyIndex :type Integer) (bFromSweep :type Boolean) (SweepResult :type Hit%20Result%20Structure%20%28by%20ref%29))
  (CallFunction|ActivatePickup OtherActor))

(event EventBeginPlay
  (|CallParentFunction)
  (Variables|Default|SetInitialLocation (Transformation|GetWorldLocation (Variables|Default|GetStaticMesh))))

(event Collision|EventActorBeginOverlap
  (params (OtherActor :type Actor%20Object%20Reference))
  (|CallParentFunction OtherActor) ; This node is disabled and will not be called.\nDrag off pins to build functionality.
)

(event EventTick
  (params (DeltaSeconds :type Float%20%28single-precision%29))
  (if (Variables|Default|GetIsRotate)
    (CallFunction|FloatandRotate DeltaSeconds)
    (|CallParentFunction DeltaSeconds)))

(fn ConstructionScript
  (bind _color (Variables|Default|GetColor))
  (bind _color_2 (Variables|Default|GetColor))
  (bind (_weapon _ammo _potion _bombs) (Utilities|Struct|BreakS_PickupColors _color))
  (bind (_weapon_2 _ammo_2 _potion_2 _bombs_2) (Utilities|Struct|BreakS_PickupColors _color_2))
  (|CallParentFunction)
  (for (_array_element _array_index) (Rendering|Material|GetMaterials (Variables|Default|GetStaticMesh))
    (bind _returnvalue (Rendering|Material|CreateDynamicMaterialInstance _array_element "None" "None" :!class /Script/Engine.KismetMaterialLibrary))
    (Rendering|Material|SetMaterial (Variables|Default|GetStaticMesh) _array_index _returnvalue)
    (Rendering|Material|SetVectorParameterValue _returnvalue "Color" (Utilities|Select :Index (Variables|Default|GetType) :NewEnumerator0 _weapon_2 :NewEnumerator1 _ammo_2 :NewEnumerator2 _potion_2 :NewEnumerator3 _bombs_2) :!class /Script/Engine.MaterialInstanceDynamic))
  (Effects|Components|ParticleSystem|SetColorParameter (Variables|Default|GetGlowingEffect) "ParticalColor" (Utilities|Select :Index (Variables|Default|GetType) :NewEnumerator0 _weapon :NewEnumerator1 _ammo :NewEnumerator2 _potion :NewEnumerator3 _bombs)))

(fn FloatandRotate
  (params (DeltaSeconds :type Float%20%28double-precision%29))
  (bind _initiallocation (Variables|Default|GetInitialLocation))
  (Utilities|FlowControl|Sequence
    (:then_0
      (if (not (Math|Float|NearlyEqual(Float) (LocalVariables|GetL_AlphaCurrent) (Math|Float|SelectFloat (LocalVariables|GetL_AlphaTarget) (LocalVariables|GetL_AlphaStart) (LocalVariables|GetL_AlphaForward)) 0.05))
        (LocalVariables|SetL_AlphaCurrent (Math|Float|ClampAngle (Math|Float|SelectFloat (+ (LocalVariables|GetL_AlphaCurrent) DeltaSeconds) (- (LocalVariables|GetL_AlphaCurrent) DeltaSeconds) (LocalVariables|GetL_AlphaForward)) 0.0 1.0))
        (else
          (LocalVariables|SetL_AlphaForward (not (LocalVariables|GetL_AlphaForward)))))
      (Transformation|SetWorldLocation (Variables|Default|GetStaticMesh) (Math|Interpolation|Ease "EaseInOut" (LocalVariables|GetL_AlphaCurrent) (Variables|Default|GetInitialLocation) (Math|Vector|MakeVector (.x _initiallocation) (.y _initiallocation) (+ (.z _initiallocation) (LocalVariables|GetL_LocationOffsetZ))) 2.0) false false))
    (:then_1
      (Transformation|AddRelativeRotation (Variables|Default|GetStaticMesh) (Math|Rotator|MakeRotator 0.0 0.0 (Variables|Default|GetRotationSpeed)) false false))))