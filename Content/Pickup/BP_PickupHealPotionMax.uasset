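; Heal potion pickup that adds potion charges to the potion bag component of the actor collecting it.
; ActivatePickupEffect looks up BPAC_PotionBag on the target and, if it is not already at max, increases its value by a fixed amount, clamped to max.
; It returns the result of that increase, or false when the bag is full or missing.
; Despite the Max in its name, it leaves the bag's maximum unchanged.
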(event EventBeginPlay
  (|CallParentFunction) ; This node is disabled and will not be called.\nDrag off pins to build functionality.
)

(event Collision|EventActorBeginOverlap
  (params (OtherActor :type Actor%20Object%20Reference))
  (|CallParentFunction OtherActor) ; This node is disabled and will not be called.\nDrag off pins to build functionality.
)

(event EventTick
  (params (DeltaSeconds :type Float%20%28single-precision%29))
  (|CallParentFunction DeltaSeconds) ; This node is disabled and will not be called.\nDrag off pins to build functionality.
)

(fn ConstructionScript
  (|CallParentFunction))

(fn ActivatePickupEffect
  (params (TargetActor :type Actor%20Object%20Reference))
  (bind _output_get (LocalVariables|SetL_PotionBag (Actor|GetComponentbyClass TargetActor "/Game/Components/BPAC_PotionBag.BPAC_PotionBag_C")))
  (Utilities|IsValid _output_get
    (:Is%20Valid
      (if (not (== (Default|GetCurValue (LocalVariables|GetL_PotionBag)) (Variables|/Game/Components/BPAC_EntityResourse.BPAC_EntityResourse_C|GetMaxValue (LocalVariables|GetL_PotionBag))))
        (bind _success (Default|IncreaseValue (LocalVariables|GetL_PotionBag) 3.0 true))
        (return _success)
        (else
          (return false))))
    (:Is%20Not%20Valid
      (return false))))