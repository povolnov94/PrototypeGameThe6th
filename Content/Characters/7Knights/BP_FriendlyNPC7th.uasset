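; Friendly NPC for the 7th knight, with trigger-zone prompt and line-by-line dialogue tied to a quest.
; Each Talk hides the Plane, then advances a lazily created WBP_NPCDialogue with a talk montage, or closes it after the last line.
; Reaching the last line updates "Find and Talk with 7th" once through the player's BPAC_QuestManager.
; Leaving the zone hides the prompt; if dialogue exists, it also resets it and appends a unique dismissive line.
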(event OnComponentEndOverlap(TriggerZone)
  (params (OverlappedComponent :type Primitive%20Component%20Object%20Reference) (OtherActor :type Actor%20Object%20Reference) (OtherComp :type Primitive%20Component%20Object%20Reference) (OtherBodyIndex :type Integer))
  (bind _uidialogue (Variables|Default|GetUIDialogue))
  (Rendering|SetVisibility (Variables|Default|GetWidget) false false)
  (Utilities|IsValid _uidialogue
    (:Is%20Valid
      (Widget|SetVisibility _uidialogue "Hidden")
      (Variables|Default|SetTalkIndex -1)
      (Utilities|Array|AddUnique (Variables|Default|GetDialogue) "why u are still here?!"))))

(event OnComponentBeginOverlap(TriggerZone)
  (params (OverlappedComponent :type Primitive%20Component%20Object%20Reference) (OtherActor :type Actor%20Object%20Reference) (OtherComp :type Primitive%20Component%20Object%20Reference) (OtherBodyIndex :type Integer) (bFromSweep :type Boolean) (SweepResult :type Hit%20Result%20Structure%20%28by%20ref%29))
  (Rendering|SetVisibility (Variables|Default|GetWidget) true false))

(event EventTalk
  (bind _returnvalue (Game|GetPlayerCharacter 0))
  (bind _returnvalue_2 (Actor|GetComponentbyClass _returnvalue "/Game/Components/BPAC_QuestManager.BPAC_QuestManager_C"))
  (Rendering|SetVisibility (Variables|Default|GetPlane) false false)
  (if (>= (Variables|Default|GetTalkIndex) (- (Utilities|Array|Length (Variables|Default|GetDialogue)) 1))
    (Widget|SetVisibility (Variables|Default|GetUIDialogue) "Hidden")
    (Variables|Default|SetTalkIndex -1)
    (else
      (Math|Integer|IncrementInt (Variables|Default|GetTalkIndex)
        (:%20%20
          (if (< (Variables|Default|GetTalkIndex) (Utilities|Array|Length (Variables|Default|GetDialogue)))
            (Variables|Default|GetUIDialogue
              (:then
                (if (Widget|IsVisible (Variables|Default|GetUIDialogue))
                  _
                  (else
                    (Widget|SetVisibility (Variables|Default|GetUIDialogue) "Visible"))))
              (:else
                (bind _returnvalue_3 (UserInterface|CreateWidget "/Game/Widgets/Dialogue/WBP_NPCDialogue.WBP_NPCDialogue_C" (Game|GetPlayerController 0)))
                (bind _output_get (Variables|Default|SetUIDialogue _returnvalue_3))
                (UserInterface|Viewport|AddtoViewport _output_get 0)))
            (Rendering|Components|TextRender|SetText (Variables|/Game/Widgets/Dialogue/WBP_NPCDialogue.WBP_NPCDialogue_C|GetTalkText (Variables|Default|GetUIDialogue)) (Utilities|Text|ToText(String) (Utilities|Array|Get(acopy) (Variables|Default|GetDialogue) (Variables|Default|GetTalkIndex))))
            (Animation|PlayAnimMontage "/Game/Characters/7Knights/AM_Talk.AM_Talk" 1.0 "None")
            (if (== (Variables|Default|GetTalkIndex) (Utilities|Array|LastIndex (Variables|Default|GetDialogue)))
              (Utilities|FlowControl|DoOnce false
                (:Completed
                  (Utilities|IsValid _returnvalue_2
                    (:Is%20Valid
                      (Default|UpdateQuest _returnvalue_2 "Find and Talk with 7th"))))))))))))

(fn ConstructionScript)

(fn InteractionInterface
  (params (Interactor :type Actor%20Object%20Reference))
  (return false))