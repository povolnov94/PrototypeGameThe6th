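; Mage NPC that guides the player through quest stages by dialogue, teleporting between spawn points as the story advances.
; Talk switches on NPCState, shows three-line dialogue in a widget, then casts a poof effect, updates the quest and relocates or finally destroys itself.
; Stages reveal jump pads, fire a finished-talk dispatcher, give bombs and a red key, and save the game, with alternate lines after a load.
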(event OnComponentEndOverlap(TriggerZone)
  (params (OverlappedComponent :type Primitive%20Component%20Object%20Reference) (OtherActor :type Actor%20Object%20Reference) (OtherComp :type Primitive%20Component%20Object%20Reference) (OtherBodyIndex :type Integer))
  (bind _uidialogue (Variables|Default|GetUIDialogue))
  (Rendering|SetVisibility (Variables|Default|GetWidget) false false)
  (Utilities|IsValid _uidialogue
    (:Is%20Valid
      (Widget|SetVisibility _uidialogue "Hidden"))))

(event OnComponentBeginOverlap(TriggerZone)
  (params (OverlappedComponent :type Primitive%20Component%20Object%20Reference) (OtherActor :type Actor%20Object%20Reference) (OtherComp :type Primitive%20Component%20Object%20Reference) (OtherBodyIndex :type Integer) (bFromSweep :type Boolean) (SweepResult :type Hit%20Result%20Structure%20%28by%20ref%29))
  (Rendering|SetVisibility (Variables|Default|GetWidget) true false))

(event EventBeginPlay
  (bind _asbp_game_instance (Utilities|Casting|CastToBP_GameInstance (Game|GetGameInstance)))
  (Variables|/Game/PlayerCharacter/BP_GameInstance.BP_GameInstance_C|SetMageNPC _asbp_game_instance self)
  (if (Variables|/Game/PlayerCharacter/BP_GameInstance.BP_GameInstance_C|GetIsGameLoad _asbp_game_instance)
    (Default|TransferNPCData _asbp_game_instance)))

(event EventTalk
  (bind _returnvalue (Game|GetPlayerCharacter 0))
  (bind _returnvalue_2 (Actor|GetComponentbyClass _returnvalue "/Game/Components/BPAC_KeyChain.BPAC_KeyChain_C"))
  (Rendering|SetVisibility (Variables|Default|GetWidget) false false)
  (switch Utilities|FlowControl|Switch|SwitchonENUM_MageState (Variables|Default|GetNPCState)
    (:NewEnumerator0
      (Rendering|SetVisibility (Variables|Default|GetPlane) false false)
      (if (>= (Variables|Default|GetTalkIndex) (- (Utilities|Array|Length (Variables|Default|GetDialogue)) 1))
        (Widget|SetVisibility (Variables|Default|GetUIDialogue) "Hidden")
        (else
          (Math|Integer|IncrementInt (Variables|Default|GetTalkIndex)
            (:%20%20
              (if (< (Variables|Default|GetTalkIndex) (Utilities|Array|Length (Variables|Default|GetDialogue)))
                (Variables|Default|GetUIDialogue
                  (:then
                    (if (Widget|IsVisible (Variables|Default|GetUIDialogue))
                      _
                      (else
                        (Widget|SetVisibility (Variables|Default|GetUIDialogue) "Visible"))))
                  (:else
                    (bind _returnvalue_3 (UserInterface|CreateWidget "/Game/Widgets/Dialogue/WBP_NPCDialogue.WBP_NPCDialogue_C" (Game|GetPlayerController 0) "The 3rd"))
                    (bind _output_get (Variables|Default|SetUIDialogue _returnvalue_3))
                    (UserInterface|Viewport|AddtoViewport _output_get 0)))
                (Rendering|Components|TextRender|SetText (Variables|/Game/Widgets/Dialogue/WBP_NPCDialogue.WBP_NPCDialogue_C|GetTalkText (Variables|Default|GetUIDialogue)) (Utilities|Text|ToText(String) (Utilities|Array|Get(acopy) (Variables|Default|GetDialogue) (Variables|Default|GetTalkIndex))))
                (Animation|PlayAnimMontage "/Game/Characters/FriendlyNPC/AM_Talk.AM_Talk" 1.0 "None")
                (if (== (Variables|Default|GetTalkIndex) (Utilities|Array|LastIndex (Variables|Default|GetDialogue)))
                  (Utilities|FlowControl|DoOnce false
                    (:Completed
                      (bind _returnvalue_4 (Animation|PlayAnimMontage "/Game/Characters/FriendlyNPC/AM_MageSpellCast.AM_MageSpellCast" 1.0 "None"))
                      (Utilities|FlowControl|Delay (- _returnvalue_4 0.2))
                      (Components|Activation|Activate (Variables|Default|GetNS_Poof) false)
                      (Utilities|FlowControl|Delay 0.3)
                      (CallFunction|SetNewSpawnPosition)
                      (for _array_element (Variables|Default|GetJumpPads)
                        (Utilities|IsValid _array_element
                          (:Is%20Valid
                            (Rendering|SetActorHiddenInGame _array_element false)
                            (CallFunction|UpdateQuest "Use magic books for come inside Mage's room")
                            (Variables|Default|SetNPCState "NewEnumerator1")
                            (CallFunction|UpdateNPCVisabilityonNewPosition)
                            (Variables|Default|SetTalkIndex -1)))))))))))))
    (:NewEnumerator1
      (CallFunction|SetNewDialogeLines "I see you've handled my books well, 6th! 8th from the future upgraded your crossbow, integrating it with future automatic weaponry" "Hurry and test it on the targets." "By the way, you can find additional ammunition in the chests!")
      (Rendering|SetVisibility (Variables|Default|GetPlane) false false)
      (if (>= (Variables|Default|GetTalkIndex) (- (Utilities|Array|Length (Variables|Default|GetDialogue)) 1))
        (Widget|SetVisibility (Variables|Default|GetUIDialogue) "Hidden")
        (else
          (Math|Integer|IncrementInt (Variables|Default|GetTalkIndex)
            (:%20%20
              (if (< (Variables|Default|GetTalkIndex) (Utilities|Array|Length (Variables|Default|GetDialogue)))
                (Variables|Default|GetUIDialogue
                  (:then
                    (if (Widget|IsVisible (Variables|Default|GetUIDialogue))
                      _
                      (else
                        (Widget|SetVisibility (Variables|Default|GetUIDialogue) "Visible"))))
                  (:else
                    (bind _returnvalue_5 (UserInterface|CreateWidget "/Game/Widgets/Dialogue/WBP_NPCDialogue.WBP_NPCDialogue_C" (Game|GetPlayerController 0)))
                    (bind _output_get_2 (Variables|Default|SetUIDialogue _returnvalue_5))
                    (UserInterface|Viewport|AddtoViewport _output_get_2 0)))
                (Rendering|Components|TextRender|SetText (Variables|/Game/Widgets/Dialogue/WBP_NPCDialogue.WBP_NPCDialogue_C|GetTalkText (Variables|Default|GetUIDialogue)) (Utilities|Text|ToText(String) (Utilities|Array|Get(acopy) (Variables|Default|GetDialogue) (Variables|Default|GetTalkIndex))))
                (Animation|PlayAnimMontage "/Game/Characters/FriendlyNPC/AM_Talk.AM_Talk" 1.0 "None")
                (if (== (Variables|Default|GetTalkIndex) (Utilities|Array|LastIndex (Variables|Default|GetDialogue)))
                  (Utilities|FlowControl|DoOnce false
                    (:Completed
                      (bind _returnvalue_6 (Animation|PlayAnimMontage "/Game/Characters/FriendlyNPC/AM_MageSpellCast.AM_MageSpellCast" 1.0 "None"))
                      (Utilities|FlowControl|Delay (- _returnvalue_6 0.2))
                      (Components|Activation|Activate (Variables|Default|GetNS_Poof) false)
                      (Utilities|FlowControl|Delay 0.2)
                      (CallFunction|SetNewSpawnPosition 1)
                      (CallFunction|UpdateQuest "Destroy targets for get the key")
                      (Default|CallOnFinishedTalk)
                      (Variables|Default|SetNPCState "NewEnumerator2")
                      (CallFunction|UpdateNPCVisabilityonNewPosition)
                      (Variables|Default|SetTalkIndex -1))))))))))
    (:NewEnumerator2
      (CallFunction|SetNewDialogeLines "I sense the chill of death - the skeletons are getting close!" "Here, take these bombs, I've enchanted them so they can't harm you." "But use them only in dire situations, you have only a few!”")
      (Rendering|SetVisibility (Variables|Default|GetPlane) false false)
      (if (>= (Variables|Default|GetTalkIndex) (- (Utilities|Array|Length (Variables|Default|GetDialogue)) 1))
        (Widget|SetVisibility (Variables|Default|GetUIDialogue) "Hidden")
        (else
          (Math|Integer|IncrementInt (Variables|Default|GetTalkIndex)
            (:%20%20
              (if (< (Variables|Default|GetTalkIndex) (Utilities|Array|Length (Variables|Default|GetDialogue)))
                (Variables|Default|GetUIDialogue
                  (:then
                    (if (Widget|IsVisible (Variables|Default|GetUIDialogue))
                      _
                      (else
                        (Widget|SetVisibility (Variables|Default|GetUIDialogue) "Visible"))))
                  (:else
                    (bind _returnvalue_7 (UserInterface|CreateWidget "/Game/Widgets/Dialogue/WBP_NPCDialogue.WBP_NPCDialogue_C" (Game|GetPlayerController 0)))
                    (bind _output_get_3 (Variables|Default|SetUIDialogue _returnvalue_7))
                    (UserInterface|Viewport|AddtoViewport _output_get_3 0)))
                (Rendering|Components|TextRender|SetText (Variables|/Game/Widgets/Dialogue/WBP_NPCDialogue.WBP_NPCDialogue_C|GetTalkText (Variables|Default|GetUIDialogue)) (Utilities|Text|ToText(String) (Utilities|Array|Get(acopy) (Variables|Default|GetDialogue) (Variables|Default|GetTalkIndex))))
                (Animation|PlayAnimMontage "/Game/Characters/FriendlyNPC/AM_Talk.AM_Talk" 1.0 "None")
                (if (== (Variables|Default|GetTalkIndex) (Utilities|Array|LastIndex (Variables|Default|GetDialogue)))
                  (Utilities|FlowControl|DoOnce false
                    (:Completed
                      (bind _returnvalue_8 (Animation|PlayAnimMontage "/Game/Characters/FriendlyNPC/AM_MageSpellCast.AM_MageSpellCast" 1.0 "None"))
                      (Utilities|FlowControl|Delay (- _returnvalue_8 0.2))
                      (Components|Activation|Activate (Variables|Default|GetNS_Poof) false)
                      (Utilities|FlowControl|Delay 0.2)
                      (Game|SpawnActorfromClass "/Game/Pickup/BP_PickupBombMax.BP_PickupBombMax_C" (Transformation|GetActorTransform self) "Undefined" "MultiplyWithRoot" 0 "NewEnumerator3" 2.0 0)
                      (Utilities|IsValid _returnvalue_2
                        (:Is%20Valid
                          (Default|AddKey _returnvalue_2 "/Game/Gameplay/Keys/BPO_Key_Red.BPO_Key_Red_C")
                          (CallFunction|SetNewSpawnPosition 2)
                          (CallFunction|UpdateQuest "Head to the main hallway")
                          (Variables|Default|SetNPCState "NewEnumerator3")
                          (CallFunction|UpdateNPCVisabilityonNewPosition)
                          (Variables|Default|SetTalkIndex -1))))))))))))
    (:NewEnumerator3
      (bind _asbp_game_instance (Utilities|Casting|CastToBP_GameInstance (Game|GetGameInstance)))
      (bind _output_get_4 (Variables|Default|SetGameInstance _asbp_game_instance))
      (if (not (Variables|/Game/PlayerCharacter/BP_GameInstance.BP_GameInstance_C|GetIsGameLoad _output_get_4))
        (CallFunction|SetNewDialogeLines "Sixth, I won't be able to assist you in the battle as I've nearly exhausted my powers." "But if things go awry..." "I'll try to teleport us through time so we can win those vile skeletons !")
        (Default|SavePlayerSGO (Variables|Default|GetGameInstance))
        (Rendering|SetVisibility (Variables|Default|GetPlane) false false)
        (if (>= (Variables|Default|GetTalkIndex) (- (Utilities|Array|Length (Variables|Default|GetDialogue)) 1))
          (Widget|SetVisibility (Variables|Default|GetUIDialogue) "Hidden")
          (else
            (Math|Integer|IncrementInt (Variables|Default|GetTalkIndex)
              (:%20%20
                (if (< (Variables|Default|GetTalkIndex) (Utilities|Array|Length (Variables|Default|GetDialogue)))
                  (Variables|Default|GetUIDialogue
                    (:then
                      (if (Widget|IsVisible (Variables|Default|GetUIDialogue))
                        _
                        (else
                          (Widget|SetVisibility (Variables|Default|GetUIDialogue) "Visible"))))
                    (:else
                      (bind _returnvalue_9 (UserInterface|CreateWidget "/Game/Widgets/Dialogue/WBP_NPCDialogue.WBP_NPCDialogue_C" (Game|GetPlayerController 0)))
                      (bind _output_get_5 (Variables|Default|SetUIDialogue _returnvalue_9))
                      (UserInterface|Viewport|AddtoViewport _output_get_5 0)))
                  (Rendering|Components|TextRender|SetText (Variables|/Game/Widgets/Dialogue/WBP_NPCDialogue.WBP_NPCDialogue_C|GetTalkText (Variables|Default|GetUIDialogue)) (Utilities|Text|ToText(String) (Utilities|Array|Get(acopy) (Variables|Default|GetDialogue) (Variables|Default|GetTalkIndex))))
                  (Animation|PlayAnimMontage "/Game/Characters/FriendlyNPC/AM_Talk.AM_Talk" 1.0 "None")
                  (if (== (Variables|Default|GetTalkIndex) (Utilities|Array|LastIndex (Variables|Default|GetDialogue)))
                    (Utilities|FlowControl|DoOnce false
                      (:Completed
                        (bind _returnvalue_10 (Animation|PlayAnimMontage "/Game/Characters/FriendlyNPC/AM_MageSpellCast.AM_MageSpellCast" 1.0 "None"))
                        (Utilities|FlowControl|Delay (- _returnvalue_10 0.2))
                        (Components|Activation|Activate (Variables|Default|GetNS_Poof) false)
                        (Utilities|FlowControl|Delay 0.2)
                        (CallFunction|SetNewSpawnPosition 3)
                        (CallFunction|UpdateQuest "Find Skeleton Capitain")
                        (Variables|Default|SetNPCState "NewEnumerator4")
                        (CallFunction|UpdateNPCVisabilityonNewPosition)
                        (Variables|Default|SetTalkIndex -1)))))))))
        (else
          (CallFunction|SetNewDialogeLines "6th, you're lucky that I had enough spatial energy to bring you back to this moment in time." "I've also replenished your supplies to make it a bit easier for you to deal with the skeletons." "Be cautious, as I'm not certain I'll be able to bring you back here again!")
          (Default|SavePlayerSGO (Variables|Default|GetGameInstance))
          (Rendering|SetVisibility (Variables|Default|GetPlane) false false)
          (if (>= (Variables|Default|GetTalkIndex) (- (Utilities|Array|Length (Variables|Default|GetDialogue)) 1))
            (Widget|SetVisibility (Variables|Default|GetUIDialogue) "Hidden")
            (else
              (Math|Integer|IncrementInt (Variables|Default|GetTalkIndex)
                (:%20%20
                  (if (< (Variables|Default|GetTalkIndex) (Utilities|Array|Length (Variables|Default|GetDialogue)))
                    (Variables|Default|GetUIDialogue
                      (:then
                        (if (Widget|IsVisible (Variables|Default|GetUIDialogue))
                          _
                          (else
                            (Widget|SetVisibility (Variables|Default|GetUIDialogue) "Visible"))))
                      (:else
                        (bind _returnvalue_11 (UserInterface|CreateWidget "/Game/Widgets/Dialogue/WBP_NPCDialogue.WBP_NPCDialogue_C" (Game|GetPlayerController 0)))
                        (bind _output_get_6 (Variables|Default|SetUIDialogue _returnvalue_11))
                        (UserInterface|Viewport|AddtoViewport _output_get_6 0)))
                    (Rendering|Components|TextRender|SetText (Variables|/Game/Widgets/Dialogue/WBP_NPCDialogue.WBP_NPCDialogue_C|GetTalkText (Variables|Default|GetUIDialogue)) (Utilities|Text|ToText(String) (Utilities|Array|Get(acopy) (Variables|Default|GetDialogue) (Variables|Default|GetTalkIndex))))
                    (Animation|PlayAnimMontage "/Game/Characters/FriendlyNPC/AM_Talk.AM_Talk" 1.0 "None")
                    (if (== (Variables|Default|GetTalkIndex) (Utilities|Array|LastIndex (Variables|Default|GetDialogue)))
                      (Utilities|FlowControl|DoOnce false
                        (:Completed
                          (bind _returnvalue_12 (Animation|PlayAnimMontage "/Game/Characters/FriendlyNPC/AM_MageSpellCast.AM_MageSpellCast" 1.0 "None"))
                          (Utilities|FlowControl|Delay (- _returnvalue_12 0.2))
                          (Components|Activation|Activate (Variables|Default|GetNS_Poof) false)
                          (Utilities|FlowControl|Delay 0.2)
                          (CallFunction|SetNewSpawnPosition 3)
                          (CallFunction|UpdateQuest "Find Skeleton Capitain")
                          (Variables|Default|SetNPCState "NewEnumerator4")
                          (CallFunction|UpdateNPCVisabilityonNewPosition)
                          (Variables|Default|SetTalkIndex -1))))))))))))
    (:NewEnumerator4
      (bind _asbp_game_instance_2 (Utilities|Casting|CastToBP_GameInstance (Game|GetGameInstance)))
      (bind _output_get_7 (Variables|Default|SetGameInstance _asbp_game_instance_2))
      (if (not (Variables|/Game/PlayerCharacter/BP_GameInstance.BP_GameInstance_C|GetIsGameLoad _output_get_7))
        (CallFunction|SetNewDialogeLines "I watched your battle with Morban's minions, 6th!" "Morban is heading to the Crypt of the Skeleton Lord. Hurry, stop him!" "Quickly check chests before you leave, there might be something useful for the fight!")
        (Rendering|SetVisibility (Variables|Default|GetPlane) false false)
        (Default|SavePlayerSGO (Variables|Default|GetGameInstance))
        (if (>= (Variables|Default|GetTalkIndex) (- (Utilities|Array|Length (Variables|Default|GetDialogue)) 1))
          (Widget|SetVisibility (Variables|Default|GetUIDialogue) "Hidden")
          (else
            (Math|Integer|IncrementInt (Variables|Default|GetTalkIndex)
              (:%20%20
                (if (< (Variables|Default|GetTalkIndex) (Utilities|Array|Length (Variables|Default|GetDialogue)))
                  (Variables|Default|GetUIDialogue
                    (:then
                      (if (Widget|IsVisible (Variables|Default|GetUIDialogue))
                        _
                        (else
                          (Widget|SetVisibility (Variables|Default|GetUIDialogue) "Visible"))))
                    (:else
                      (bind _returnvalue_13 (UserInterface|CreateWidget "/Game/Widgets/Dialogue/WBP_NPCDialogue.WBP_NPCDialogue_C" (Game|GetPlayerController 0)))
                      (bind _output_get_8 (Variables|Default|SetUIDialogue _returnvalue_13))
                      (UserInterface|Viewport|AddtoViewport _output_get_8 0)))
                  (Rendering|Components|TextRender|SetText (Variables|/Game/Widgets/Dialogue/WBP_NPCDialogue.WBP_NPCDialogue_C|GetTalkText (Variables|Default|GetUIDialogue)) (Utilities|Text|ToText(String) (Utilities|Array|Get(acopy) (Variables|Default|GetDialogue) (Variables|Default|GetTalkIndex))))
                  (Animation|PlayAnimMontage "/Game/Characters/FriendlyNPC/AM_Talk.AM_Talk" 1.0 "None")
                  (if (== (Variables|Default|GetTalkIndex) (Utilities|Array|LastIndex (Variables|Default|GetDialogue)))
                    (Utilities|FlowControl|DoOnce false
                      (:Completed
                        (bind _returnvalue_14 (Animation|PlayAnimMontage "/Game/Characters/FriendlyNPC/AM_MageSpellCast.AM_MageSpellCast" 1.0 "None"))
                        (Utilities|FlowControl|Delay (- _returnvalue_14 0.2))
                        (Components|Activation|Activate (Variables|Default|GetNS_Poof) false)
                        (Utilities|FlowControl|Delay 0.2)
                        (CallFunction|UpdateQuest "Find Skeleton Capitain on the bridge!")
                        (Actor|DestroyActor)
                        (Variables|Default|SetTalkIndex -1)))))))))
        (else
          (CallFunction|SetNewDialogeLines "6th, you're lucky that I had enough spatial energy to bring you back to this moment in time." "I've also replenished your supplies to make it a bit easier for you to deal with the skeletons." "Be cautious, as I'm not certain I'll be able to bring you back here again!")
          (Default|SavePlayerSGO (Variables|Default|GetGameInstance))
          (Rendering|SetVisibility (Variables|Default|GetPlane) false false)
          (if (>= (Variables|Default|GetTalkIndex) (- (Utilities|Array|Length (Variables|Default|GetDialogue)) 1))
            (Widget|SetVisibility (Variables|Default|GetUIDialogue) "Hidden")
            (else
              (Math|Integer|IncrementInt (Variables|Default|GetTalkIndex)
                (:%20%20
                  (if (< (Variables|Default|GetTalkIndex) (Utilities|Array|Length (Variables|Default|GetDialogue)))
                    (Variables|Default|GetUIDialogue
                      (:then
                        (if (Widget|IsVisible (Variables|Default|GetUIDialogue))
                          _
                          (else
                            (Widget|SetVisibility (Variables|Default|GetUIDialogue) "Visible"))))
                      (:else
                        (bind _returnvalue_15 (UserInterface|CreateWidget "/Game/Widgets/Dialogue/WBP_NPCDialogue.WBP_NPCDialogue_C" (Game|GetPlayerController 0)))
                        (bind _output_get_9 (Variables|Default|SetUIDialogue _returnvalue_15))
                        (UserInterface|Viewport|AddtoViewport _output_get_9 0)))
                    (Rendering|Components|TextRender|SetText (Variables|/Game/Widgets/Dialogue/WBP_NPCDialogue.WBP_NPCDialogue_C|GetTalkText (Variables|Default|GetUIDialogue)) (Utilities|Text|ToText(String) (Utilities|Array|Get(acopy) (Variables|Default|GetDialogue) (Variables|Default|GetTalkIndex))))
                    (Animation|PlayAnimMontage "/Game/Characters/FriendlyNPC/AM_Talk.AM_Talk" 1.0 "None")
                    (if (== (Variables|Default|GetTalkIndex) (Utilities|Array|LastIndex (Variables|Default|GetDialogue)))
                      (Utilities|FlowControl|DoOnce false
                        (:Completed
                          (bind _returnvalue_16 (Animation|PlayAnimMontage "/Game/Characters/FriendlyNPC/AM_MageSpellCast.AM_MageSpellCast" 1.0 "None"))
                          (Utilities|FlowControl|Delay (- _returnvalue_16 0.2))
                          (Components|Activation|Activate (Variables|Default|GetNS_Poof) false)
                          (Utilities|FlowControl|Delay 0.2)
                          (CallFunction|UpdateQuest "Find Skeleton Capitain on the bridge!")
                          (Actor|DestroyActor)
                          (Variables|Default|SetTalkIndex -1))))))))))))))

(fn ConstructionScript)

(fn InteractionInterface
  (params (Interactor :type Actor%20Object%20Reference))
  (return false))

(fn SetNewDialogeLines
  (params (DialogeLine1 :type String) (DialogeLine2 :type String) (DialogeLine3 :type String))
  (Utilities|Array|SetArrayElem (Variables|Default|GetDialogue) 0 DialogeLine1)
  (Utilities|Array|SetArrayElem (Variables|Default|GetDialogue) 1 DialogeLine2)
  (Utilities|Array|SetArrayElem (Variables|Default|GetDialogue) 2 DialogeLine3))

(fn SetNewSpawnPosition
  (params (PositionIndex :type Integer%20%28by%20ref%29))
  (Transformation|SetActorLocation (Transformation|GetActorLocation (Utilities|Array|Get(acopy) (Variables|Default|GetSpawnPoints) PositionIndex)) false false)
  (Transformation|SetActorRotation (Transformation|GetActorRotation (Utilities|Array|Get(acopy) (Variables|Default|GetSpawnPoints) PositionIndex)))
  (Rendering|Material|SetMaterial (Variables|Character|GetMesh) 0 "/Engine/VREditor/UI/DiscMaterial.DiscMaterial"))

(fn UpdateQuest
  (params (CurrentQuest :type String%20%28by%20ref%29))
  (bind _returnvalue (Game|GetPlayerCharacter 0))
  (bind _returnvalue_2 (Actor|GetComponentbyClass _returnvalue "/Game/Components/BPAC_QuestManager.BPAC_QuestManager_C"))
  (Utilities|IsValid _returnvalue_2
    (:Is%20Valid
      (Default|UpdateQuest _returnvalue_2 CurrentQuest))))

(fn UpdateNPCVisabilityonNewPosition
  (bind _uidialogue (Variables|Default|GetUIDialogue))
  (Rendering|Material|SetMaterial (Variables|Character|GetMesh) 0 "/Game/Assets/Mage/mage_texture1.mage_texture1")
  (Rendering|SetVisibility (Variables|Default|GetPlane) true false)
  (Rendering|SetVisibility (Variables|Default|GetWidget) false false)
  (Utilities|IsValid _uidialogue
    (:Is%20Valid
      (Widget|SetVisibility _uidialogue "Hidden"))))