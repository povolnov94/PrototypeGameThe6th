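; Trigger volume that starts the Morban Skullcleaver boss fight with a cutscene and a quest update.
; Any overlap of its box fetches player 0's character rather than the overlapping actor, shows WBP_BossFightCutscene and updates that character's quest objective.
; It binds to the widget's start and finish events, and on finish fires its cutscene-finished dispatcher and destroys itself.
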(event OnComponentBeginOverlap(Box)
  (params (OverlappedComponent :type Primitive%20Component%20Object%20Reference) (OtherActor :type Actor%20Object%20Reference) (OtherComp :type Primitive%20Component%20Object%20Reference) (OtherBodyIndex :type Integer) (bFromSweep :type Boolean) (SweepResult :type Hit%20Result%20Structure%20%28by%20ref%29))
  (bind _asbp_third_person_character (Utilities|Casting|CastToBP_ThirdPersonCharacter (Game|GetPlayerCharacter 0)))
  (bind _output_get (Variables|Default|SetPlayerCharacter _asbp_third_person_character))
  (Utilities|IsValid _output_get
    (:Is%20Valid
      (bind _returnvalue (UserInterface|CreateWidget "/Game/Widgets/WBP_BossFightCutscene.WBP_BossFightCutscene_C"))
      (EventDispatchers|BindEventtoOnCutSceneStarted _returnvalue (EventDispatchers|CreateEvent (Variables|Default|GetPlayerCharacter) :!event SetIMCItroCutscene))
      (EventDispatchers|BindEventtoOnCutSceneFinished _returnvalue (EventDispatchers|CreateEvent (Variables|Default|GetPlayerCharacter) :!event SetIMCGamemode))
      (EventDispatchers|BindEventtoOnCutSceneFinished _returnvalue (delegate Custom|CustomEvent))
      (UserInterface|Viewport|AddtoViewport _returnvalue 0)
      (Default|UpdateQuest (Variables|/Game/Characters/BP_ThirdPersonCharacter.BP_ThirdPersonCharacter_C|GetBPAC_QuestManager (Variables|Default|GetPlayerCharacter)) "Defeat \"Morban Skullcleaver\"!"))))

(event Custom|CustomEvent
  (Default|CallOnCutscenefinished)
  (Actor|DestroyActor))

(fn ConstructionScript)