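; BP_TriggerWaveMode is a box trigger that starts wave mode in what appears to be the main hall.
; On overlap it shows a cutscene widget and updates the player character's quest to killing all skeletons to open the castle gate.
; When the cutscene finishes, a DoOnce-guarded event adds the wave HUD widget, calls NewWave on the game mode and destroys the trigger.
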(event OnComponentBeginOverlap(Box)
  (params (OverlappedComponent :type Primitive%20Component%20Object%20Reference) (OtherActor :type Actor%20Object%20Reference) (OtherComp :type Primitive%20Component%20Object%20Reference) (OtherBodyIndex :type Integer) (bFromSweep :type Boolean) (SweepResult :type Hit%20Result%20Structure%20%28by%20ref%29))
  (bind _asbp_third_person_character (Utilities|Casting|CastToBP_ThirdPersonCharacter (Game|GetPlayerCharacter 0)))
  (bind _output_get (Variables|Default|SetPlayerCharacter _asbp_third_person_character))
  (Utilities|IsValid _output_get
    (:Is%20Valid
      (bind _returnvalue (UserInterface|CreateWidget "/Game/Widgets/WBP_MainhallCutscene.WBP_MainhallCutscene_C"))
      (EventDispatchers|BindEventtoOnCutSceneStarted _returnvalue (EventDispatchers|CreateEvent (Variables|Default|GetPlayerCharacter) :!event SetIMCItroCutscene))
      (EventDispatchers|BindEventtoOnCutSceneFinished _returnvalue (EventDispatchers|CreateEvent (Variables|Default|GetPlayerCharacter) :!event SetIMCGamemode))
      (EventDispatchers|BindEventtoOnCutSceneFinished _returnvalue (delegate Custom|CustomEvent))
      (UserInterface|Viewport|AddtoViewport _returnvalue 0)
      (Default|UpdateQuest (Variables|/Game/Characters/BP_ThirdPersonCharacter.BP_ThirdPersonCharacter_C|GetBPAC_QuestManager (Variables|Default|GetPlayerCharacter)) "Kill all Skeletons for open the castle gate!"))))

(event Custom|CustomEvent
  (Utilities|FlowControl|DoOnce false
    (:Completed
      (bind _asbp_third_person_game_mode (Utilities|Casting|CastToBP_ThirdPersonGameMode (Game|GetGameMode)))
      (bind _returnvalue (UserInterface|CreateWidget "/Game/Widgets/WaveMode/WBP_WaveMode.WBP_WaveMode_C"))
      (bind _output_get (Variables|Default|SetWaveWidget _returnvalue))
      (UserInterface|Viewport|AddtoViewport _output_get 0)
      (Default|NewWave _asbp_third_person_game_mode)
      (Actor|DestroyActor))))

(fn ConstructionScript)