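; BP_MagicWall is an environment magic wall that can be switched on and off, built from a Plane component and a Niagara effect.
; Activate sets the plane's collision to QueryAndProbe and starts the effect without a reset.
; Deactivate disables the collision and stops the effect.
; BeginPlay calls Deactivate, so the wall starts inactive until something calls Activate.
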(event Custom|Activate
  (Collision|SetCollisionEnabled (Variables|Default|GetPlane) "QueryAndProbe")
  (Components|Activation|Activate (Variables|Default|GetNiagara) false))

(event Custom|Deactivate
  (Collision|SetCollisionEnabled (Variables|Default|GetPlane) "NoCollision")
  (Components|Activation|Deactivate (Variables|Default|GetNiagara)))

(event EventBeginPlay
  (CallFunction|Deactivate))

(fn ConstructionScript)