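; Interactable loot chest that swings open and closed, dropping its loot only once through the BPACDropLoot component.
; Its overlap box manages interaction-queue membership and a tooltip, while the interaction interface toggles Open and Close.
; Current and target states gate both actions as a timeline, rate-scaled to AnimDuration, rotates the lid and commits the target state on finish.
; Tick prints the current state on screen for debugging.
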(event OnComponentBeginOverlap(IntteractBox)
  (params (OverlappedComponent :type Primitive%20Component%20Object%20Reference) (OtherActor :type Actor%20Object%20Reference) (OtherComp :type Primitive%20Component%20Object%20Reference) (OtherBodyIndex :type Integer) (bFromSweep :type Boolean) (SweepResult :type Hit%20Result%20Structure%20%28by%20ref%29))
  (CallFunction|AddtoInteractionQueue self OtherActor)
  (if (Utilities|Enum|Equal(Enum) (Variables|Default|GetCurrentState) "NewEnumerator1")
    (Rendering|SetVisibility (Variables|Default|Get%20TooltipWidget) true false)))

(event OnComponentEndOverlap(IntteractBox)
  (params (OverlappedComponent :type Primitive%20Component%20Object%20Reference) (OtherActor :type Actor%20Object%20Reference) (OtherComp :type Primitive%20Component%20Object%20Reference) (OtherBodyIndex :type Integer))
  (CallFunction|RemovefromInteractionQueue self OtherActor)
  (Rendering|SetVisibility (Variables|Default|Get%20TooltipWidget) false false))

(event EventTick
  (params (DeltaSeconds :type Float%20%28single-precision%29))
  (Development|PrintString (Utilities|String|ToString(Text) (Utilities|Text|FormatText "{Name} State is {State}" (Utilities|GetObjectName self) (Utilities|String|EnumtoString (Variables|Default|GetCurrentState)))) true false "(R=1.000000,G=0.000000,B=0.139645,A=1.000000)" DeltaSeconds))

(event EventBeginPlay
  (Components|Timeline|SetPlayRate (Variables|Default|GetOpenTimeline) (Math|Float|SafeDivide (Components|Timeline|GetTimelineLength (Variables|Default|GetOpenTimeline)) (Variables|Default|GetAnimDuration))))

(fn ConstructionScript)

(fn Close
  (Utilities|SwitchCurrentState
    (:Opened
      (Variables|Default|SetCurrentState "NewEnumerator3"))
    (:Closed
      (return false))
    (:Locked
      (return false))
    (:InAction
      (Utilities|SwitchTargetState
        (:Opened
          _)
        (:Closed
          (return false))
        (:Locked
          (return false))
        (:InAction
          (return false)))))
  (Variables|Default|SetTargetState "NewEnumerator1")
  (Components|Timeline|ReversefromEnd (Variables|Default|GetOpenTimeline))
  (return true))

(fn Open
  (Utilities|SwitchCurrentState
    (:Opened
      (return false))
    (:Closed
      (Variables|Default|SetCurrentState "NewEnumerator3"))
    (:Locked
      (return false))
    (:InAction
      (Utilities|SwitchTargetState
        (:Opened
          (return false))
        (:Closed
          _)
        (:Locked
          (return false))
        (:InAction
          (return false)))))
  (Variables|Default|SetTargetState "NewEnumerator0")
  (Components|Timeline|PlayfromStart (Variables|Default|GetOpenTimeline))
  (bind _success (CallFunction|DropLoot))
  (return _success))

(fn AnimationOpen
  (params (AnimProgress :type Float%20%28double-precision%29))
  (Transformation|SetRelativeRotation (Variables|Default|GetRotator) (Math|Rotator|MakeRotator (* (Variables|Default|GetMaxOpenAngle) AnimProgress) 0.0 0.0) false false))

(fn DropLoot
  (if (not (Variables|/Game/Components/BPAC_DropLoot.BPAC_DropLoot_C|GetIsDroped (Variables|Default|GetBPAC_DropLoot)))
    (Default|DropLoot (Variables|Default|GetBPAC_DropLoot))
    (bind _success (Default|SetIsDropped (Variables|Default|GetBPAC_DropLoot)))
    (return _success)
    (else
      (return false))))

(fn InteractionInterface
  (params (Interactor :type Actor%20Object%20Reference))
  (Utilities|SwitchCurrentState
    (:Opened
      (CallFunction|Close)
      (Rendering|SetVisibility (Variables|Default|Get%20TooltipWidget) true false)
      (return true))
    (:Closed
      (CallFunction|Open)
      (Rendering|SetVisibility (Variables|Default|Get%20TooltipWidget) false false)
      (return true))
    (:InAction
      (return false))))