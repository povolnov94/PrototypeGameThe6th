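; Base door Blueprint that opens, closes and locks by tracking Opened, Closed, Locked and InAction states, starting from a configurable initial state.
; Open and Close set a target state and play DoorTimeline, whose rate is scaled to AnimDuration, restarting it from either end if reversed mid-motion.
; The Animation function yaws the Rotator up to MaxOpenAngle.
; SetIsLocked only locks a closed door or unlocks a locked one, subject to BPACLock approval.
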(event EventBeginPlay
  (Components|Timeline|SetPlayRate (Variables|Default|GetDoorTimeline) (Math|Float|SafeDivide (Components|Timeline|GetTimelineLength (Variables|Default|GetDoorTimeline)) (Variables|Default|GetAnimDuration))))

(event EventTick
  (params (DeltaSeconds :type Float%20%28single-precision%29)))

(fn ConstructionScript
  (Variables|State|SetInitialState (select (Utilities|Enum|Equal(Enum) (Variables|State|GetInitialState) "NewEnumerator3") "NewEnumerator1" (Variables|State|GetInitialState)))
  (bind _output_get (Variables|State|SetCurrentState (Variables|State|GetInitialState)))
  (CallFunction|Animation (Utilities|Select :Index _output_get :NewEnumerator0 1.0 :NewEnumerator1 0.0 :NewEnumerator2 0.0 :NewEnumerator3 0.0))
  (Variables|/Game/Components/BPAC_Lock.BPAC_Lock_C|SetIsLocked (Variables|Default|GetBPAC_Lock) (Utilities|Enum|Equal(Enum) (Variables|State|GetCurrentState) "NewEnumerator2")))

(fn Close
  (Utilities|SwitchCurrentState
    (:Opened
      (Variables|State|SetCurrentState "NewEnumerator3"))
    (:Closed
      (return false))
    (:Locked
      (return false))
    (:InAction
      (Utilities|SwitchTargetState
        (:Opened
          _)
        (:Closed
          (return false))
        (:Locked
          (return false))
        (:InAction
          (return false)))))
  (Variables|State|SetTargetState "NewEnumerator1")
  (Components|Timeline|ReversefromEnd (Variables|Default|GetDoorTimeline))
  (return true))

(fn Open
  (Utilities|SwitchCurrentState
    (:Opened
      (return false))
    (:Closed
      (Variables|State|SetCurrentState "NewEnumerator3"))
    (:Locked
      (return false))
    (:InAction
      (Utilities|SwitchTargetState
        (:Opened
          (return false))
        (:Closed
          _)
        (:Locked
          (return false))
        (:InAction
          (return false)))))
  (Variables|State|SetTargetState "NewEnumerator0")
  (Components|Timeline|PlayfromStart (Variables|Default|GetDoorTimeline))
  (return true))

(fn Animation
  (params (AnimProgress :type Float%20%28double-precision%29))
  (Transformation|SetRelativeRotation (Variables|Default|GetRotator) (Math|Rotator|MakeRotator 0.0 0.0 (* (Variables|Default|GetMaxOpenAngle) AnimProgress)) false false))

(fn GetCurrentState
  (return (Variables|State|GetCurrentState)))

(fn GetTargetState
  (return (Variables|State|GetTargetState)))

(fn SetIsLocked
  (params (OtherActor :type Actor%20Object%20Reference) (IsLocked :type Boolean))
  (if IsLocked
    (if (Utilities|Enum|Equal(Enum) (Variables|State|GetCurrentState) "NewEnumerator1")
      (bind _success (Default|Lock (Variables|Default|GetBPAC_Lock) OtherActor))
      (if _success
        (Variables|State|SetCurrentState "NewEnumerator2")
        (return true)
        (else
          (return false)))
      (else
        (return false)))
    (elif (Utilities|Enum|Equal(Enum) (Variables|State|GetCurrentState) "NewEnumerator2")
      (bind _success_2 (Default|Unlock (Variables|Default|GetBPAC_Lock) OtherActor))
      (if _success_2
        (Variables|State|SetCurrentState "NewEnumerator1")
        (return true)
        (else
          (return false)))
      (else
        (return false)))))