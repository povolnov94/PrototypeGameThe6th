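; BP_TrapSpikes is a spike trap actor that damages actors overlapping its spikes.
; Any overlap with BoxCollision starts a short delay, then teleports the Spikes component upward by a fixed offset and lowers it again after a second delay.
; The Spikes component's own overlap event applies damage from the Amount variable to the other actor, independently of the trigger sequence.
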(event OnComponentBeginOverlap(BoxCollision)
  (params (OverlappedComponent :type Primitive%20Component%20Object%20Reference) (OtherActor :type Actor%20Object%20Reference) (OtherComp :type Primitive%20Component%20Object%20Reference) (OtherBodyIndex :type Integer) (bFromSweep :type Boolean) (SweepResult :type Hit%20Result%20Structure%20%28by%20ref%29))
  (bind _spikes (Variables|Default|Getspikes))
  (bind _spikes_2 (Variables|Default|Getspikes))
  (bind _returnvalue (Transformation|GetWorldLocation _spikes_2))
  (bind _returnvalue_2 (Transformation|GetWorldLocation _spikes))
  (Utilities|FlowControl|Delay 0.5)
  (Transformation|SetWorldLocation _spikes_2 (Math|Vector|MakeVector (.x _returnvalue) (.y _returnvalue) (+ (.z _returnvalue) 194.0)) false false)
  (Utilities|FlowControl|Delay 1.5)
  (Transformation|SetWorldLocation _spikes (Math|Vector|MakeVector (.x _returnvalue_2) (.y _returnvalue_2) (- (.z _returnvalue_2) 194.0)) false false))

(event OnComponentBeginOverlap(spikes)
  (params (OverlappedComponent :type Primitive%20Component%20Object%20Reference) (OtherActor :type Actor%20Object%20Reference) (OtherComp :type Primitive%20Component%20Object%20Reference) (OtherBodyIndex :type Integer) (bFromSweep :type Boolean) (SweepResult :type Hit%20Result%20Structure%20%28by%20ref%29))
  (Game|Damage|ApplyDamage OtherActor (Variables|Default|GetAmount) 0 0))

(event EventBeginPlay)

(event Collision|EventActorBeginOverlap
  (params (OtherActor :type Actor%20Object%20Reference)))

(event EventTick
  (params (DeltaSeconds :type Float%20%28single-precision%29)))

(fn ConstructionScript)