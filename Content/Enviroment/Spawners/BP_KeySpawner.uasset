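; BP_KeySpawner is a spawner that places an actor, presumably a key, once enough designated targets have been killed.
; On BeginPlay it binds to the OnValueZero event of each target's BPAC_Health component.
; Each event increments a kill counter, and a count of exactly three spawns ActorTospawn at the Box component's location, regardless of how many targets are listed.
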(event Custom|CustomEvent
  (Variables|Default|SetTargetsKilled (+ (Variables|Default|GetTargetsKilled) 1))
  (if (== (Variables|Default|GetTargetsKilled) 3)
    (Game|SpawnActorfromClass (Variables|Default|GetActorTospawn) (Math|Transform|MakeTransform (Transformation|GetWorldLocation (Variables|Default|GetBox)) "0, 0, 0" "1.000000,1.000000,1.000000") "AdjustIfPossibleButAlwaysSpawn" "MultiplyWithRoot" 0 0)))

(event EventBeginPlay
  (for _array_element (Variables|Default|GetTargetsToKill)
    (EventDispatchers|BindEventtoOnValueZero (Actor|GetComponentbyClass _array_element "/Game/Components/BPAC_Health.BPAC_Health_C") (delegate Custom|CustomEvent))))

(fn ConstructionScript)