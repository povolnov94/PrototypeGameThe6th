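; BP_EnemySpawner is an enemy spawner actor that periodically creates enemies at its own transform.
; Activate starts a looping 15-second timer that calls SpawnEnemy on each tick; nothing runs at BeginPlay.
; SpawnEnemy randomly picks a self-bomb enemy or a minion, spawns it with adjusted collision handling, and returns true if the spawn is valid.
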(event Custom|TryToSpawn
  (CallFunction|SpawnEnemy))

(event Custom|Activate
  (Utilities|Time|SetTimerbyEvent (delegate Custom|TryToSpawn) 15.0 true))

(event EventBeginPlay)

(fn ConstructionScript)

(fn SpawnEnemy
  (bind _returnvalue (Game|SpawnActorfromClass (Utilities|Select :Index (Math|Random|RandomIntegerinRange 0 1) :Option%200 "/Game/Enemy/BP_EnemySelfBomb.BP_EnemySelfBomb_C" :Option%201 "/Game/Enemy/BP_EnemyMinion.BP_EnemyMinion_C") (Transformation|GetActorTransform) "AdjustIfPossibleButAlwaysSpawn" "MultiplyWithRoot" 0 0))
  (if (Utilities|IsValid _returnvalue)
    (return true)))