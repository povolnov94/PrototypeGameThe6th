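; Base actor for area-of-effect magick spells that damages actors within a radius of its location.
; Trigger runs either externally or automatically after a short delay on BeginPlay, performing a one-shot sphere overlap on a single object type, optionally ignoring the instigator.
; Each overlapped actor is broadcast through the OnAOEOverlapActor dispatcher, then receives base damage.
; The debug-sphere toggle currently has no effect because its drawing node is disconnected.
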(event Custom|SpawnAOESphere
  (if (Variables|Default|GetDrawDebugSphere)
    _
    (else
      _))
  (bind _outactors (Collision|SphereOverlapActors (Transformation|GetActorLocation) (Variables|Default|GetRadius) (Utilities|Array|MakeArray "ObjectTypeQuery7") 0 (select (Variables|Default|GetIgnoreInstigator) (Utilities|Array|MakeArray (Game|GetInstigator)) 0)))
  (for _array_element _outactors
    (Default|CallOnAOEOverlapActor _array_element)
    (Game|Damage|ApplyDamage _array_element (Variables|Default|GetBaseDamage) 0 0)))

(event Custom|Trigger
  (CallFunction|SpawnAOESphere))

(event EventBeginPlay
  (if (Variables|Default|GetTriggerOnBeginPlay)
    (Utilities|FlowControl|Delay 0.2)
    (CallFunction|Trigger)))

(fn ConstructionScript)