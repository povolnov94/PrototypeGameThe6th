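; BP_Bomb is a timed bomb actor that explodes three seconds after BeginPlay.
; The explosion spawns a Niagara effect at the mesh's relative location, applies fixed damage to every actor overlapping its Sphere, fires a RadialForce impulse, then destroys the bomb.
; An older particle emitter spawn remains in the graph but never runs.
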(event Custom|Explode
  (Niagara|SpawnSystematLocation "/Game/Art/FVX/NS_ExplosionBomb.NS_ExplosionBomb" (Variables|/Script/Engine.SceneComponent|GetRelativeLocation (Variables|Default|GetStaticMesh)))
  (for _array_element (Collision|GetOverlappingActors (Variables|Default|GetSphere) 0 :!class /Script/Engine.PrimitiveComponent)
    (Game|Damage|ApplyDamage _array_element 8e+01 0 0))
  (Class|RadialForceComponent|FireImpulse (Variables|Default|GetRadialForce))
  (Actor|DestroyActor))

(event EventBeginPlay
  (Utilities|FlowControl|Delay 3.0)
  (CallFunction|Explode))

(fn ConstructionScript)