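; Ammo pack pickup that refills ammo for one weapon class carried by the actor that takes it.
; Overlap handling is left to the parent pickup, while this child supplies ActivatePickupEffect.
; The effect finds the target's BPAC_WeaponManeger component, looks up the weapon matching WeaponClass and calls AddAmmo on it.
; It returns false when the manager or weapon is missing or current ammo equals the maximum, and true once ammo is added.
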(event EventBeginPlay
  (|CallParentFunction) ; This node is disabled and will not be called.\nDrag off pins to build functionality.
)

(event Collision|EventActorBeginOverlap
  (params (OtherActor :type Actor%20Object%20Reference))
  (|CallParentFunction OtherActor))

(event EventTick
  (params (DeltaSeconds :type Float%20%28single-precision%29))
  (|CallParentFunction DeltaSeconds) ; This node is disabled and will not be called.\nDrag off pins to build functionality.
)

(fn ConstructionScript
  (|CallParentFunction))

(fn ActivatePickupEffect
  (params (TargetActor :type Actor%20Object%20Reference))
  (bind _output_get (LocalVariables|SetL_WeaponManager (Actor|GetComponentbyClass TargetActor "/Game/Components/BPAC_WeaponManeger.BPAC_WeaponManeger_C")))
  (Utilities|IsValid _output_get
    (:Is%20Valid
      (if (Utilities|Array|ContainsItem (Variables|/Game/Components/BPAC_WeaponManeger.BPAC_WeaponManeger_C|GetWeaponClasses (LocalVariables|GetL_WeaponManager)) (Variables|Default|GetWeaponClass))
        (if (== (Utilities|Struct|BreakS_WeaponData (Variables|/Game/Weapons/BaseClasses/BP_BaseWeapon.BP_BaseWeapon_C|GetWeaponData (Utilities|Array|Get(acopy) (Variables|/Game/Components/BPAC_WeaponManeger.BPAC_WeaponManeger_C|GetWeapons (LocalVariables|GetL_WeaponManager)) (Utilities|Array|FindItem (Variables|/Game/Components/BPAC_WeaponManeger.BPAC_WeaponManeger_C|GetWeaponClasses (LocalVariables|GetL_WeaponManager)) (Variables|Default|GetWeaponClass))))) (Utilities|Struct|BreakS_WeaponData (Variables|/Game/Weapons/BaseClasses/BP_BaseWeapon.BP_BaseWeapon_C|GetWeaponData (Utilities|Array|Get(acopy) (Variables|/Game/Components/BPAC_WeaponManeger.BPAC_WeaponManeger_C|GetWeapons (LocalVariables|GetL_WeaponManager)) (Utilities|Array|FindItem (Variables|/Game/Components/BPAC_WeaponManeger.BPAC_WeaponManeger_C|GetWeaponClasses (LocalVariables|GetL_WeaponManager)) (Variables|Default|GetWeaponClass))))))
          (return false)
          (else
            (Default|AddAmmo (Utilities|Array|Get(acopy) (Variables|/Game/Components/BPAC_WeaponManeger.BPAC_WeaponManeger_C|GetWeapons (LocalVariables|GetL_WeaponManager)) (Utilities|Array|FindItem (Variables|/Game/Components/BPAC_WeaponManeger.BPAC_WeaponManeger_C|GetWeaponClasses (LocalVariables|GetL_WeaponManager)) (Variables|Default|GetWeaponClass))))
            (return true)))
        (else
          (return false))))
    (:Is%20Not%20Valid
      (return false))))