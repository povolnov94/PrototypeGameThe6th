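; Shotgun weapon Blueprint that fires several projectiles per shot, using one round from the clip.
; MakeShot line-traces from the owner's camera, or eye viewpoint as fallback, to find the aim direction from the muzzle, then updates ammo and widget.
; The spawn loop starts at index 3, giving projectiles random cone rotations but one shared Direction.
; The cone axis is built from the muzzle socket's location components rather than its rotation.
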(event EventBeginPlay
  (|CallParentFunction) ; This node is disabled and will not be called.\nDrag off pins to build functionality.
)

(event Collision|EventActorBeginOverlap
  (params (OtherActor :type Actor%20Object%20Reference))
  (|CallParentFunction OtherActor) ; This node is disabled and will not be called.\nDrag off pins to build functionality.
)

(event EventTick
  (params (DeltaSeconds :type Float%20%28single-precision%29))
  (|CallParentFunction DeltaSeconds) ; This node is disabled and will not be called.\nDrag off pins to build functionality.
)

(fn ConstructionScript
  (|CallParentFunction))

(fn MakeShot
  (bind _returnvalue (Components|GetOwner))
  (bind _weapondata (Variables|Default|GetWeaponData))
  (bind _muzzlefx (Variables|Default|GetMuzzleFX))
  (bind _muzzlefxsocketname (Variables|Default|GetMuzzleFXSocketName))
  (bind (_projectileclass _damage) (Utilities|Struct|BreakS_WeaponData _weapondata))
  (bind (_outlocation _outrotation) (Actor|GetActorEyesViewPoint _returnvalue))
  (bind _returnvalue_2 (Transformation|GetSocketLocation _muzzlefx _muzzlefxsocketname))
  (if (> (.CurrentClipAmmo (Utilities|Struct|BreakS_WeaponData (Variables|Default|GetWeaponData))) 0)
    (Utilities|IsValid (Variables|Default|GetOwnerCamera)
      (:Is%20Valid
        (bind _desiredview (Class|CameraComponent|GetCameraView (Variables|Default|GetOwnerCamera) 0.0))
        (LocalVariables|SetL_StartPoint (.Location (Utilities|Struct|BreakMinimalViewInfo _desiredview)))
        (LocalVariables|SetL_EndPoint (+ (LocalVariables|GetL_StartPoint) (* (Math|Rotator|GetRotationXVector (.Rotation (Utilities|Struct|BreakMinimalViewInfo _desiredview))) (Variables|Default|GetTraceLengh)))))
      (:Is%20Not%20Valid
        (LocalVariables|SetL_StartPoint _outlocation)
        (LocalVariables|SetL_EndPoint (+ (LocalVariables|GetL_StartPoint) (* (Math|Rotator|GetRotationXVector _outrotation) (Variables|Default|GetTraceLengh))))))
    (bind (_outhit _returnvalue_3) (Collision|LineTraceByChannel (LocalVariables|GetL_StartPoint) (LocalVariables|GetL_EndPoint) "TraceTypeQuery2" false (Utilities|Array|MakeArray (Components|GetOwner)) "ForDuration" false "(R=1.000000,G=0.000000,B=0.000000,A=1.000000)" "(R=0.000000,G=1.000000,B=0.000000,A=1.000000)" 2.0))
    (LocalVariables|SetL_OutHit _outhit)
    (LocalVariables|SetL_Direction (Math|Vector|Normalize (- (Math|Vector|SelectVector (.ImpactPoint (Collision|BreakHitResult (LocalVariables|GetL_OutHit))) (.TraceEnd (Collision|BreakHitResult (LocalVariables|GetL_OutHit))) _returnvalue_3) (Transformation|GetSocketLocation (Variables|Default|GetWeaponMesh) (Variables|Default|GetMuzzleFXSocketName)))))
    (CallFunction|OnMakeShot (LocalVariables|GetL_OutHit))
    (Utilities|Struct|SetmembersinS_WeaponData (Variables|Default|GetWeaponData) (Math|Integer|Max(Integer) (- (.CurrentClipAmmo (Utilities|Struct|BreakS_WeaponData (Variables|Default|GetWeaponData))) 1)))
    (CallFunction|UpdateWidget)
    (for _index (range 3 (Variables|Default|GetBulletsInShot))
      (LocalVariables|SetL_Index _index)
      (Game|SpawnActorfromClass _projectileclass (Math|Transform|MakeTransform (Transformation|GetSocketLocation (Variables|Default|GetMuzzleFX) (Variables|Default|GetMuzzleFXSocketName)) (CallFunction|GetSprayAngle (Math|Vector|GetForwardVector (Math|Rotator|MakeRotator (.x _returnvalue_2) (.y _returnvalue_2) (.z _returnvalue_2))) (Variables|Default|GetShotAngle))) "AdjustIfPossibleButAlwaysSpawn" "MultiplyWithRoot" 0 (LocalVariables|GetL_Direction) _damage 0))))

(fn GetSprayAngle
  (params (MuzzleDirection :type Vector) (MaxAngle :type Float%20%28double-precision%29))
  (return (Math|Rotator|MakeRotfromX (Math|Random|RandomUnitVectorinConeinDegrees MuzzleDirection MaxAngle))))

(fn UpdateWidget
  (|CallParentFunction))