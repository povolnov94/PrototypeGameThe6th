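; Crossbow weapon Blueprint that extends a parent weapon's reload with a visible, droppable ammo mesh.
; Starting a reload detaches the mesh, enables physics so it falls away and sets a short timer, calling the parent only if the mesh is valid.
; Reload snaps the same mesh back onto the weapon's ammo socket, visible and without collision.
; DestroyAmmoPack only hides the mesh for reuse, as its destroy call is unconnected.
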(event EventBeginPlay
  (|CallParentFunction) ; This node is disabled and will not be called.\nDrag off pins to build functionality.
)

(event Collision|EventActorBeginOverlap
  (params (OtherActor :type Actor%20Object%20Reference))
  (|CallParentFunction OtherActor) ; This node is disabled and will not be called.\nDrag off pins to build functionality.
)

(event EventTick
  (params (DeltaSeconds :type Float%20%28single-precision%29))
  (|CallParentFunction DeltaSeconds) ; This node is disabled and will not be called.\nDrag off pins to build functionality.
)

(fn ConstructionScript
  (|CallParentFunction))

(fn Reload
  (|CallParentFunction)
  (Transformation|AttachComponentToComponent (Variables|Default|GetStaticMesh1) (Variables|Default|GetStaticMesh) "AmmoSocket" "SnapToTarget" "SnapToTarget" "SnapToTarget" true)
  (Rendering|SetVisibility (Variables|Default|GetStaticMesh1) true false)
  (Collision|SetCollisionEnabled (Variables|Default|GetStaticMesh1) "NoCollision"))

(fn DestroyAmmoPack
  (Rendering|SetVisibility (Variables|Default|GetStaticMesh1) false false))

(fn StartReloading
  (if (Utilities|IsValid (Variables|Default|GetStaticMesh1))
    (Transformation|DetachFromComponent (Variables|Default|GetStaticMesh1) "KeepWorld" "KeepWorld" "KeepWorld" true)
    (Collision|SetCollisionEnabled (Variables|Default|GetStaticMesh1) "QueryAndPhysics")
    (Physics|SetSimulatePhysics (Variables|Default|GetStaticMesh1) true)
    (Utilities|Time|SetTimerbyEvent (EventDispatchers|CreateEvent :!event DestroyAmmoPack) 1.5)
    (bind _success (|CallParentFunction))
    (return _success)))